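; Ground-targeted AOE cast ability that holds its montage at zero rate while a trace indicator, sized by radius and range, awaits confirmation.
; Confirmation retries targeting if already casting, or moving without instant cast; otherwise it records cast info and plays the montage at a calculated rate.
; The montage's Event.Cast.Execute event makes the server commit, play cast sound and pass target data to OnConfirm.
; Cancellation interrupts the character's cast.
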(event Ability|EventActivateAbility
  (bind _radius (Variables|Default|GetRadius))
  (bind _abilitydata (Variables|Default|GetAbilityData))
  (bind _abilitydata_2 (Variables|Default|GetAbilityData))
  (bind _abilitysound (Variables|/Script/PROJ.AbilityData|GetAbilitySound _abilitydata_2))
  (bind _abilitysound_2 (Variables|/Script/PROJ.AbilityData|GetAbilitySound _abilitydata))
  (Utilities|FlowControl|Sequence
    (:then_0
      (if (not (GameplayTags|HasMatchingGameplayTag (Ability|GetAbilitySystemComponentfromActorInfo) "(TagName=\"State.Casting\")"))
        (|PlayMontageandWaitProxy "None" (Variables|/Script/PROJ.AbilityData|GetMontage (Variables|Default|GetAbilityData)) 0.0 "None" true 1.0 0.0 false
          (:then
            (Utilities|IsValid _abilitysound_2
              (:Is%20Valid
                (bind _returnvalue (Audio|SpawnSoundatLocation _abilitysound_2 (Transformation|GetActorLocation (Ability|GetAvatarActorfromActorInfo)) "0, 0, 0" 1.0 1.0 0.0 0 0))
                (Class|AudioParameterControllerInterface|SetTriggerParameter _returnvalue "Start")))))))
    (:then_1
      (bind _data (|WaitTargetData :ConfirmationType "UserConfirmed" :Class "/Game/UI/Game/InGameWIdgets/AbilityIndicator/BP_GroundTrace_Indicator_WaitTargetData.BP_GroundTrace_Indicator_WaitTargetData_C" :Size (Math|Vector|MakeVector 128.0 _radius _radius) :MaxRange (Variables|Default|GetRange) :TraceProfile "(Name=\"BlockAll\")" :bTraceAffectsAimPitch false :StartLocation (Class|GameplayAbility|MakeTargetLocationInfofromOwnerActor) :ReticleClass 0 :!label _label)
        (:ValidData
          (if (GameplayTags|HasMatchingGameplayTag (Ability|GetAbilitySystemComponentfromActorInfo) "(TagName=\"State.Casting\")")
            (Development|PrintString "Hello")
            (goto _label)
            (else
              (if (Variables|Default|GetbIsInstantCast)
                _
                (elif (GameplayTags|HasMatchingGameplayTag (Ability|GetAbilitySystemComponentfromActorInfo) "(TagName=\"State.Movement.Moving\")")
                  (goto _label)
                  (else
                    _)))
              (Development|PrintString "CONFIRM")
              (bind _returnvalue_2 (Class|BaseGameplayAbility|CalculateAbilityMontagePlayRate))
              (Variables|Default|SetPlayRate _returnvalue_2)
              (CallFunction|SetCastNotify)
              (|PlayMontageandWaitProxy "None" (Variables|/Script/PROJ.AbilityData|GetMontage (Variables|Default|GetAbilityData)) (Variables|Default|GetPlayRate) "None" false 1.0 0.0 false
                (:then
                  (Ability|Tasks|WaitGameplayEvent "(TagName=\"Event.Cast.Execute\")" 0
                    (:EventReceived
                      (Ability|HasAuthority
                        (:True
                          (Ability|CommitAbility)
                          (Utilities|FlowControl|Sequence
                            (:then_0
                              (Utilities|IsValid _abilitysound
                                (:Is%20Valid
                                  (bind _returnvalue_3 (Audio|SpawnSoundatLocation _abilitysound (Transformation|GetActorLocation (Ability|GetAvatarActorfromActorInfo)) "0, 0, 0" 1.0 1.0 0.0 0 0))
                                  (Class|AudioParameterControllerInterface|SetTriggerParameter _returnvalue_3 "Cast"))))
                            (:then_1
                              (Variables|Default|SetPlayRate 0.0)
                              (Class|GACastAOE|OnConfirm _data))))))))))))
        (:Cancelled
          (Ability|CancelAbility))))))

(event Ability|EventOnEndAbility
  (params (bWasCancelled :type Boolean))
  (if bWasCancelled
    (bind _asbp_third_person_character (Utilities|Casting|CastToBP_ThirdPersonCharacter (Ability|GetAvatarActorfromActorInfo)))
    (Default|InterruptCast _asbp_third_person_character (Variables|Default|GetCastTime))))

(fn SetCastNotify
  (bind _asbp_third_person_character (Utilities|Casting|CastToBP_ThirdPersonCharacter (Ability|GetAvatarActorfromActorInfo)))
  (Variables|/Game/Characters/Base/_Core/BP_ThirdPersonCharacter.BP_ThirdPersonCharacter_C|SetCurrentCastInfo _asbp_third_person_character (Utilities|Struct|MakeS_CastInfo (Variables|Default|GetCastTime) (Variables|Default|GetAbilityName) (.millisecond (Math|DateTime|Now)))))