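; OmniShot gameplay ability that fires a five-projectile fan of light attack projectiles from the avatar's location.
; On authority, it commits the ability, then a RepeatAction task spawns the projectiles almost instantly, offsetting each one's yaw by a fixed step from the avatar's facing.
; Each projectile is initialized as an ability actor, and the ability ends when the task finishes.
; The non-authority branch does nothing, and the commit result is not checked.
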(event Ability|EventActivateAbility
  (bind _returnvalue (Ability|GetAvatarActorfromActorInfo))
  (bind _returnvalue_2 (Transformation|GetActorRotation _returnvalue))
  (Ability|HasAuthority
    (:True
      (Ability|CommitAbility)
      (bind _actionnumber (|RepeatAction 0.001 5)
        (:OnPerformAction
          (bind _returnvalue_3 (Game|SpawnActorfromClass "/Game/AbilitySystem/Abilities/PlayerClasses/LoremIpsum/LightAttack/BP_Projectile_LightAttack.BP_Projectile_LightAttack_C" (Math|Transform|MakeTransform (+ "" (Transformation|GetActorLocation _returnvalue)) (Math|Rotator|MakeRotator (.roll _returnvalue_2) (.pitch _returnvalue_2) (+ (* _actionnumber 5.0) (+ (.yaw _returnvalue_2) -1e+01)))) "Undefined" "MultiplyWithRoot" 0 0))
          (Class|BaseGameplayAbility|InitializeAbilityActor _returnvalue_3))
        (:OnFinished
          (Ability|EndAbility))))))

(event Ability|EventOnEndAbility
  (params (bWasCancelled :type Boolean)))