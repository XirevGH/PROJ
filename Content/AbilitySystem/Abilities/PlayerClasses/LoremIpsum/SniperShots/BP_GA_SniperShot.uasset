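; Sniper shot gameplay ability for the LoremIpsum player class that manages the character's HoloSight during the ability.
; Extends a parent ability's activation, then waits once for the Event.Cast.Start gameplay event to activate the avatar's HoloSight.
; Ending the ability deactivates the HoloSight.
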(event Ability|EventOnEndAbility
  (params (bWasCancelled :type Boolean))
  (bind _asbp_lorem_ipsum (Utilities|Casting|CastToBP_LoremIpsum (Ability|GetAvatarActorfromActorInfo)))
  (Components|Activation|SetActive (Variables|/Game/Characters/LoremIpsum/_Core/BP_LoremIpsum.BP_LoremIpsum_C|GetHoloSight _asbp_lorem_ipsum) false false))

(event EventActivateAbility
  (|CallParentFunction)
  (bind _asbp_lorem_ipsum (Utilities|Casting|CastToBP_LoremIpsum (Ability|GetAvatarActorfromActorInfo)))
  (Ability|Tasks|WaitGameplayEvent "(TagName=\"Event.Cast.Start\")" 0 true
    (:EventReceived
      (Components|Activation|SetActive (Variables|/Game/Characters/LoremIpsum/_Core/BP_LoremIpsum.BP_LoremIpsum_C|GetHoloSight _asbp_lorem_ipsum) true false))))