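; BP_GA_Instant_Teleport is a Gameplay Ability that instantly moves the player forward.
; On activation with authority it commits the ability, then sets the avatar's location a fixed distance along its forward vector with a slight upward offset.
; The move uses teleport physics without sweeping, so obstacles in the path are not checked.
; It prints a debug string and ends the ability immediately afterwards.
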(event Ability|EventActivateAbility
  (bind _returnvalue (Ability|GetAvatarActorfromActorInfo))
  (Ability|HasAuthority
    (:True
      (Ability|CommitAbility)
      (Transformation|SetActorLocation _returnvalue (+ (Transformation|GetActorLocation _returnvalue) (+ (* (Transformation|GetActorForwardVector _returnvalue) 5e+02) "0.000000,0.000000,100.000000")) false true)
      (Development|PrintString "Hello")
      (Ability|EndAbility))))

(event Ability|EventOnEndAbility
  (params (bWasCancelled :type Boolean)))