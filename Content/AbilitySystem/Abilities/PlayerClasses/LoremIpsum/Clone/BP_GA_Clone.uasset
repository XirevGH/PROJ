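; Gameplay ability that spawns a clone of the player's avatar at a targeted location.
; Activation is not overridden; the logic runs in OnConfirm when target data arrives.
; On authority only, it commits the ability, spawns an actor of the avatar's class at the target end point with a hard-coded upward offset, then ends.
; The CommitAbility result is not checked before spawning.
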(event Ability|EventActivateAbility
  (|CallParentFunction) ; This node is disabled and will not be called.\nDrag off pins to build functionality.
)

(event Ability|EventOnEndAbility
  (params (bWasCancelled :type Boolean)))

(event EventOnConfirm
  (params (Data :type Gameplay%20Ability%20Target%20Data%20Handle%20Structure%20%28by%20ref%29))
  (Ability|HasAuthority
    (:True
      (Ability|CommitAbility)
      (Game|SpawnActorfromClass (Utilities|GetClass (Ability|GetAvatarActorfromActorInfo)) (Math|Conversions|ToTransform(Vector) (+ (Class|AbilitySystemBlueprintLibrary|GetTargetDataEndPoint Data) "0.000000,0.000000,100.000000")) "Undefined" "MultiplyWithRoot" 0 0)
      (Ability|EndAbility))))