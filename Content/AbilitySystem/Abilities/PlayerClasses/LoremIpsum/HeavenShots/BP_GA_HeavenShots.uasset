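; BP_GA_HeavenShots is a gameplay ability that drops a short volley of light-attack projectiles from above a targeted point.
; On confirm, the authority commits the ability, storing but not branching on the result, then runs a RepeatAction task.
; Each repeat spawns a downward-facing BP_Projectile_LightAttack above the target data end point and initializes it as an ability actor.
; The ability ends when the repeats finish.
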(event Ability|EventActivateAbility
  (|CallParentFunction) ; This node is disabled and will not be called.\nDrag off pins to build functionality.
)

(event Ability|EventOnEndAbility
  (params (bWasCancelled :type Boolean)))

(event EventOnConfirm
  (params (Data :type Gameplay%20Ability%20Target%20Data%20Handle%20Structure%20%28by%20ref%29))
  (Ability|HasAuthority
    (:True
      (bind _returnvalue (Ability|CommitAbility))
      (Variables|Default|SetbHasCommit _returnvalue)
      (|RepeatAction 0.2 3
        (:OnPerformAction
          (bind _returnvalue_2 (Game|SpawnActorfromClass "/Game/AbilitySystem/Abilities/PlayerClasses/LoremIpsum/LightAttack/BP_Projectile_LightAttack.BP_Projectile_LightAttack_C" (Math|Transform|MakeTransform (+ (Class|AbilitySystemBlueprintLibrary|GetTargetDataEndPoint Data) "0.000000,0.000000,350.000000") (Math|Rotator|MakeRotator 0.0 -9e+01 0.0)) "Undefined" "MultiplyWithRoot" 0 0))
          (Class|BaseGameplayAbility|InitializeAbilityActor _returnvalue_2))
        (:OnFinished
          (Ability|EndAbility))))))