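; Gameplay ability that teleports the Wraith player character to a targeted location.
; Activation runs the parent logic and turns on the Wraith's teleport targeting component, which switches off on the Cast.Confirm gameplay event or when the ability ends.
; On confirm, only the authority commits the ability, moves the avatar to the target data end point with a hardcoded upward offset and no sweep, then ends it.
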(event Ability|EventActivateAbility
  (|CallParentFunction)
  (bind _asbp_wraith (Utilities|Casting|CastToBP_Wraith (Ability|GetAvatarActorfromActorInfo)))
  (Components|Activation|SetActive (Variables|/Game/Characters/Wraith/_Core/BP_Wraith.BP_Wraith_C|GetP_Wraith_Teleport_Targeting _asbp_wraith) true false)
  (Ability|Tasks|WaitGameplayEvent "(TagName=\"Event.Cast.Confirm\")" 0 true
    (:EventReceived
      (bind _asbp_wraith_2 (Utilities|Casting|CastToBP_Wraith (Ability|GetAvatarActorfromActorInfo)))
      (Components|Activation|SetActive (Variables|/Game/Characters/Wraith/_Core/BP_Wraith.BP_Wraith_C|GetP_Wraith_Teleport_Targeting _asbp_wraith_2) false false))))

(event EventOnConfirm
  (params (Data :type Gameplay%20Ability%20Target%20Data%20Handle%20Structure%20%28by%20ref%29))
  (Ability|HasAuthority
    (:True
      (Ability|CommitAbility)
      (Transformation|SetActorLocation (Ability|GetAvatarActorfromActorInfo) (+ (Class|AbilitySystemBlueprintLibrary|GetTargetDataEndPoint Data) "0.000000,0.000000,100.000000") false true)
      (Ability|EndAbility))))

(event Ability|EventOnEndAbility
  (params (bWasCancelled :type Boolean))
  (|CallParentFunction bWasCancelled)
  (bind _asbp_wraith (Utilities|Casting|CastToBP_Wraith (Ability|GetAvatarActorfromActorInfo)))
  (Components|Activation|SetActive (Variables|/Game/Characters/Wraith/_Core/BP_Wraith.BP_Wraith_C|GetP_Wraith_Teleport_Targeting _asbp_wraith) false false))