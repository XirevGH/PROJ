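; Projectile for the Wraith's light attack that applies an effect to what it strikes.
; Both overlap and hit events call the parent handler, then on the server check ShouldSkipHit before applying the effect to the other actor and destroying the projectile.
; The overlap path also prints debug strings naming the other actor and the caster.
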(event EventOnBeginOverlap
  (params (OverlappedComponent :type Primitive%20Component%20Object%20Reference) (OtherActor :type Actor%20Object%20Reference) (OtherComp :type Primitive%20Component%20Object%20Reference) (OtherBodyIndex :type Integer) (bFromSweep :type Boolean) (SweepResult :type Hit%20Result%20Structure%20%28by%20ref%29))
  (|CallParentFunction OverlappedComponent OtherActor OtherComp OtherBodyIndex bFromSweep SweepResult)
  (Development|PrintString (Utilities|GetDisplayName OtherActor))
  (Development|PrintString (Utilities|String|Append "csater is " (Utilities|GetDisplayName (Variables|Default|GetCaster))))
  (Networking|SwitchHasAuthority
    (:Authority
      (bind _returnvalue (Class|AbilityActor|ShouldSkipHit OtherActor))
      (if (not _returnvalue)
        (Class|AbilityActor|ApplyEffecttoTarget OtherActor)
        (Actor|DestroyActor)))))

(event EventOnProjectileHit
  (params (HitComp :type Primitive%20Component%20Object%20Reference) (OtherActor :type Actor%20Object%20Reference) (OtherComp :type Primitive%20Component%20Object%20Reference) (NormalImpulse :type Vector :default "0, 0, 0") (Hit :type Hit%20Result%20Structure%20%28by%20ref%29))
  (|CallParentFunction HitComp OtherActor OtherComp NormalImpulse Hit)
  (Networking|SwitchHasAuthority
    (:Authority
      (bind _returnvalue (Class|AbilityActor|ShouldSkipHit OtherActor))
      (if (not _returnvalue)
        (Class|AbilityActor|ApplyEffecttoTarget OtherActor)
        (Actor|DestroyActor)))))

(fn ConstructionScript)