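; Base-style gameplay ability for the Wraith's sniper shot that toggles the character's HoloSight component during the cast.
; On activation it waits once for the Event.Cast.Start gameplay event, then activates the HoloSight on the Wraith avatar.
; When the ability ends, cancelled or not, it deactivates the HoloSight again.
; Both events call their parent implementations, so the shot logic itself lives outside this Blueprint.
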(event Ability|EventOnEndAbility
  (params (bWasCancelled :type Boolean))
  (|CallParentFunction bWasCancelled)
  (bind _asbp_lorem_ipsum (Utilities|Casting|CastToBP_Wraith (Ability|GetAvatarActorfromActorInfo)))
  (Components|Activation|SetActive (Variables|/Game/Characters/Wraith/_Core/BP_Wraith.BP_Wraith_C|GetHoloSight _asbp_lorem_ipsum) false false))

(event EventActivateAbility
  (|CallParentFunction)
  (bind _asbp_lorem_ipsum (Utilities|Casting|CastToBP_Wraith (Ability|GetAvatarActorfromActorInfo)))
  (Ability|Tasks|WaitGameplayEvent "(TagName=\"Event.Cast.Start\")" 0 true
    (:EventReceived
      (Components|Activation|SetActive (Variables|/Game/Characters/Wraith/_Core/BP_Wraith.BP_Wraith_C|GetHoloSight _asbp_lorem_ipsum) true false))))