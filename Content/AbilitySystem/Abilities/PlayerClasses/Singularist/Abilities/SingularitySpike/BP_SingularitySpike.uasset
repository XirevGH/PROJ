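; Spawned actor for the Singularist's Singularity Spike ability: a meteor strike that applies an effect to characters in its impact area.
; The first particle collision of the instant meteor latches HasLanded, unhides that effect, plays meteor audio, activates a shower particle and triggers the hit check.
; That check scans Characters overlapping the capsule, filters them through ShouldSkipHit and AlreadyHit, then applies the effect and records each target.
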(event OnParticleCollide(P_Gideon_MeteorInstant)
  (params (EventName :type Name :default "None") (EmitterTime :type Float%20%28single-precision%29) (ParticleTime :type Integer) (Location :type Vector :default "0, 0, 0") (Velocity :type Vector :default "0, 0, 0") (Direction :type Vector :default "0, 0, 0") (Normal :type Vector :default "0, 0, 0") (BoneName :type Name :default "None") (PhysMat :type Physical%20Material%20Object%20Reference))
  (if (not (Variables|Default|GetbHasLanded))
    (Variables|Default|SetbHasLanded true)
    (Development|SetHiddeninGame (Variables|Default|GetP_Gideon_MeteorInstant) false false)
    (Audio|Components|Audio|Play (Variables|Default|GetMS_Meteor) 0.0)
    (Components|Activation|Activate (Variables|Default|GetP_Gideon_Meteor_Shower1) false)
    (CallFunction|CustomEvent)))

(event OnParticleCollide(P_Gideon_Meteor_Shower)
  (params (EventName :type Name :default "None") (EmitterTime :type Float%20%28single-precision%29) (ParticleTime :type Integer) (Location :type Vector :default "0, 0, 0") (Velocity :type Vector :default "0, 0, 0") (Direction :type Vector :default "0, 0, 0") (Normal :type Vector :default "0, 0, 0") (BoneName :type Name :default "None") (PhysMat :type Physical%20Material%20Object%20Reference)))

(event Custom|CustomEvent
  (for _array_element (Collision|GetOverlappingActors (Variables|Default|GetCapsule) "/Script/Engine.Character" :!class /Script/Engine.PrimitiveComponent)
    (bind _returnvalue (Class|AbilityActor|ShouldSkipHit _array_element))
    (if (not _returnvalue)
      (if (not (Utilities|Array|ContainsItem (Variables|Default|Getalready%20hit) _array_element))
        (bind _output_get (Variables|Default|SetOther%20Actor _array_element))
        (Class|AbilityActor|ApplyEffecttoTarget _output_get)
        (Utilities|Array|Add (Variables|Default|Getalready%20hit) (Variables|Default|GetOther%20Actor))))))

(fn ConstructionScript)