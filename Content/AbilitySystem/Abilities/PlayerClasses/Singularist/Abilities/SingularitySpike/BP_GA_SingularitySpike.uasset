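; Singularist player ability that spawns a Singularity Spike actor at the targeted location.
; On confirm, the server commits the ability, spawns the actor at the target data end point transform, initializes it and ends the ability; clients just end it.
; An unconnected chain for a cast delay with cancel-on-movement is present but never runs.
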(event EventOnConfirm
  (params (Data :type Gameplay%20Ability%20Target%20Data%20Handle%20Structure%20%28by%20ref%29))
  (bind _returnvalue (Class|AbilitySystemBlueprintLibrary|GetTargetDataEndPointTransform Data))
  (Ability|HasAuthority
    (:True
      (Ability|CommitAbility)
      (bind _returnvalue_2 (Game|SpawnActorfromClass "/Game/AbilitySystem/Abilities/PlayerClasses/Singularist/Abilities/SingularitySpike/BP_SingularitySpike.BP_SingularitySpike_C" (Math|Transform|MakeTransform (.location _returnvalue) (.rotation _returnvalue) "1.000000,1.000000,1.000000") "AlwaysSpawn" "MultiplyWithRoot" 0 0))
      (Class|BaseGameplayAbility|InitializeAbilityActor _returnvalue_2)
      (Ability|EndAbility))
    (:False
      (Ability|EndAbility))))