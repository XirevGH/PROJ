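; Two-ended wormhole for the Singularist's Conjure Wormhole ability that lets characters on the caster's team teleport between its portals.
; On interaction it compares team IDs, then uses the clicked component to choose which sphere the player must overlap and which portal is the destination.
; Teleporting sets the actor's location directly and activates effects at both portals.
; A timer started on BeginPlay destroys the wormhole after its active time, spawning closing and dissolve emitters.
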(event Custom|Destroy%20Actor
  (bind _p_portal_entrance (Variables|Default|GetP_Portal_Entrance))
  (bind _p_portal_exit (Variables|Default|GetP_Portal_Exit))
  (bind _returnvalue (Transformation|GetWorldRotation _p_portal_exit))
  (bind _returnvalue_2 (Transformation|GetWorldLocation _p_portal_exit))
  (Effects|SpawnEmitteratLocation (Variables|Default|GetPortal_Entrance_Close) (Transformation|GetWorldLocation _p_portal_entrance) (Transformation|GetWorldRotation _p_portal_entrance))
  (Effects|SpawnEmitteratLocation (Variables|Default|GetPortal_Exit_Close) _returnvalue_2 _returnvalue)
  (Effects|SpawnEmitteratLocation (Variables|Default|GetRing_Dissolve) _returnvalue_2 _returnvalue)
  (Actor|DestroyActor))

(event Custom|TeleportPlayer_Event
  (params (Target%20Wormhole :type Scene%20Component%20Object%20Reference) (Player :type Actor%20Object%20Reference))
  (CallFunction|TeleportPlayer Target%20Wormhole Player)
  (Components|Activation|Activate (Variables|Default|GetP_Portal_Teleport_Enter) true)
  (Components|Activation|Activate (Variables|Default|GetP_Portal_Teleport_Exit) true))

(event EventBeginPlay
  (Utilities|Time|SetTimerbyEvent (delegate Custom|Destroy%20Actor) (Variables|Default|GetWormholeActiveTime)))

(event EventInteract
  (params (Player :type Actor%20Object%20Reference) (ClickedActorComponent :type Actor%20Component%20Object%20Reference))
  (bind _asbp_third_person_character (Utilities|Casting|CastToBP_ThirdPersonCharacter Player))
  (bind _teamid (Default|GetTeamID _asbp_third_person_character))
  (bind _asbp_third_person_character_2 (Utilities|Casting|CastToBP_ThirdPersonCharacter (Variables|Default|GetCaster)))
  (bind _teamid_2 (Default|GetTeamID _asbp_third_person_character_2))
  (if (Utilities|Enum|Equal(Enum) _teamid_2 _teamid)
    (if (== ClickedActorComponent (Variables|Default|GetClickDetactionSphere))
      (if (Utilities|Array|ContainsItem (Collision|GetOverlappingActors (Variables|Default|GetSphere) "/Script/Engine.Character" :!class /Script/Engine.PrimitiveComponent) Player)
        (CallFunction|TeleportPlayerEvent (Variables|Default|GetP_Portal_Entrance) Player))
      (elif (Utilities|Array|ContainsItem (Collision|GetOverlappingActors (Variables|Default|GetSphere1) "/Script/Engine.Character" :!class /Script/Engine.PrimitiveComponent) Player)
        (CallFunction|TeleportPlayerEvent (Variables|Default|GetP_Portal_Exit) Player)))))

(fn ConstructionScript)

(fn TeleportPlayer
  (params (TargetWormhole :type Scene%20Component%20Object%20Reference) (Player :type Actor%20Object%20Reference))
  (Transformation|SetActorLocation Player (Transformation|GetWorldLocation TargetWormhole) false true))