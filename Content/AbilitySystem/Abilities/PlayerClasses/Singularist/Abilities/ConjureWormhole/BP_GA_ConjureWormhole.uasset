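; Gameplay ability for the Singularist class that conjures a pair of linked wormholes between the player and a targeted point.
; On confirm, it spawns the wormhole actor at the character's mesh transform, initializes it as an ability actor and teleports its second wormhole component to the target data's end point.
; It stores the actor and ends the ability; the cancel event destroys that actor if still valid.
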(event EventOnCancel
  (params (Data :type Gameplay%20Ability%20Target%20Data%20Handle%20Structure%20%28by%20ref%29))
  (bind _wormholes (Variables|Default|GetWormholes))
  (Utilities|IsValid _wormholes
    (:Is%20Valid
      (Actor|DestroyActor _wormholes))))

(event EventOnConfirm
  (params (Data :type Gameplay%20Ability%20Target%20Data%20Handle%20Structure%20%28by%20ref%29))
  (bind _asbp_third_person_character (Utilities|Casting|CastToBP_ThirdPersonCharacter (Ability|GetAvatarActorfromActorInfo)))
  (bind _returnvalue (Game|SpawnActorfromClass (Variables|Default|GetWormholeClass) (Math|Transform|MakeTransform (.location (Transformation|GetWorldTransform (Variables|/Script/Engine.Character|GetMesh _asbp_third_person_character))) (.rotation (Transformation|GetWorldTransform (Variables|/Script/Engine.Character|GetMesh _asbp_third_person_character))) "1.000000,1.000000,1.000000") "AdjustIfPossibleButAlwaysSpawn" "MultiplyWithRoot" 0 0))
  (Class|BaseGameplayAbility|InitializeAbilityActor _returnvalue)
  (Transformation|SetWorldLocation (Variables|/Game/AbilitySystem/Abilities/PlayerClasses/Singularist/Abilities/ConjureWormhole/BP_Wormhole.BP_Wormhole_C|GetWormhole_2 _returnvalue) (Class|AbilitySystemBlueprintLibrary|GetTargetDataEndPoint Data) false true)
  (Variables|Default|SetWormholes _returnvalue)
  (Ability|EndAbility))