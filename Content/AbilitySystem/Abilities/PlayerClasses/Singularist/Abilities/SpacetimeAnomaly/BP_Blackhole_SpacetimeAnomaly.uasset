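; Black hole actor for the Singularist's Spacetime Anomaly ability that drags nearby characters to its center and applies an effect to them.
; Each tick, characters overlapping the pull sphere that pass the skip check move toward the center at constant speed, with sweep.
; Those reaching the center inside the damage sphere receive the effect once, tracked by an array.
; A timer ends it after the pull duration with a burst particle.
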(event Custom|Destroy%20actor
  (Rendering|SetVisibility (Variables|Default|GetP_Gideon_Ultimate) false false)
  (Effects|SpawnEmitteratLocation (Variables|Default|GetDestroy%20Particle) (Transformation|GetWorldLocation (Variables|Default|GetDefaultSceneRoot)))
  (Actor|DestroyActor))

(event Custom|PullEnemy
  (params (Delta%20Sec :type Float%20%28double-precision%29))
  (bind _alreadyappliedeffectactors (Variables|Default|GetAlreadyAppliedEffectActors))
  (for _array_element (Collision|GetOverlappingActors (Variables|Default|GetSphere) "/Script/Engine.Character" :!class /Script/Engine.PrimitiveComponent)
    (bind _returnvalue (Class|AbilityActor|ShouldSkipHit _array_element))
    (if (not _returnvalue)
      (bind _ascharacter (Utilities|Casting|CastToCharacter _array_element))
      (Utilities|IsatCenter _ascharacter _ascharacter
        (:else
          (Transformation|SetActorLocation _ascharacter (Math|Interpolation|VInterptoConstant (Transformation|GetActorLocation _ascharacter) (Transformation|GetWorldLocation (Variables|Default|GetScene)) Delta%20Sec 5e+02) true false))
        (:then
          (if (not (Utilities|Array|ContainsItem _alreadyappliedeffectactors _ascharacter))
            (Class|AbilityActor|ApplyEffecttoTarget _ascharacter)
            (Utilities|Array|Add _alreadyappliedeffectactors _ascharacter)))))))

(event EventBeginPlay
  (Utilities|Time|SetTimerbyEvent (delegate Custom|Destroy%20actor) (Variables|Default|GetPullDuration)))

(event EventTick
  (params (DeltaSeconds :type Float%20%28single-precision%29))
  (|CallParentFunction DeltaSeconds)
  (CallFunction|PullEnemy DeltaSeconds))

(fn ConstructionScript)