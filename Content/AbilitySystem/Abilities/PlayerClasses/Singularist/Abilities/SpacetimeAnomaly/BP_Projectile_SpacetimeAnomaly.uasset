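; Projectile for the Singularist's Spacetime Anomaly ability that turns into a black hole on impact.
; Both hit and overlap events call the parent logic, then on the server skip filtered actors and spawn BP_Blackhole_SpacetimeAnomaly slightly below the collision component.
; The black hole receives the caster, its ability system component and the effect specs, and the projectile then destroys itself.
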(event Custom|SpawnBlackhole
  (bind _returnvalue (Game|SpawnActorfromClass "/Game/AbilitySystem/Abilities/PlayerClasses/Singularist/Abilities/SpacetimeAnomaly/BP_Blackhole_SpacetimeAnomaly.BP_Blackhole_SpacetimeAnomaly_C" (Math|Conversions|ToTransform(Vector) (+ (Transformation|GetWorldLocation (Variables|Default|GetCollisionComp)) "0.000000,0.000000,-100.000000")) "Undefined" "MultiplyWithRoot" 0 0))
  (Class|AbilityActor|InitializeAbilityActor _returnvalue (Variables|Default|GetCaster) (Variables|Default|GetCasterASC) (Variables|Default|GetEffectSpecHandles))
  (Actor|DestroyActor))

(event EventOnProjectileHit
  (params (HitComp :type Primitive%20Component%20Object%20Reference) (OtherActor :type Actor%20Object%20Reference) (OtherComp :type Primitive%20Component%20Object%20Reference) (NormalImpulse :type Vector :default "0, 0, 0") (Hit :type Hit%20Result%20Structure%20%28by%20ref%29))
  (|CallParentFunction HitComp OtherActor OtherComp NormalImpulse Hit)
  (Networking|SwitchHasAuthority
    (:Authority
      (bind _returnvalue (Class|AbilityActor|ShouldSkipHit OtherActor))
      (if (not _returnvalue)
        (CallFunction|SpawnBlackhole)))))

(event EventOnBeginOverlap
  (params (OverlappedComponent :type Primitive%20Component%20Object%20Reference) (OtherActor :type Actor%20Object%20Reference) (OtherComp :type Primitive%20Component%20Object%20Reference) (OtherBodyIndex :type Integer) (bFromSweep :type Boolean) (SweepResult :type Hit%20Result%20Structure%20%28by%20ref%29))
  (|CallParentFunction OverlappedComponent OtherActor OtherComp OtherBodyIndex bFromSweep SweepResult)
  (Networking|SwitchHasAuthority
    (:Authority
      (bind _returnvalue (Class|AbilityActor|ShouldSkipHit OtherActor))
      (if (not _returnvalue)
        (CallFunction|SpawnBlackhole)))))

(fn ConstructionScript
  (|CallParentFunction))