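; Base projectile Blueprint that overrides ShouldSkipHit to skip hits on characters sharing the local player's team.
; It calls the parent check without using its result, then casts the hit actor to BP_ThirdPersonCharacter and reads its team ID.
; That ID is compared with player controller 0's TeamID rather than the projectile's instigator.
; Both players' names and team IDs are printed for debugging.
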(fn ConstructionScript)

(fn ShouldSkipHit
  (params (OtherActor :type Actor%20Object%20Reference))
  (|CallParentFunction OtherActor)
  (bind _asbp_third_person_character (Utilities|Casting|CastToBP_ThirdPersonCharacter OtherActor))
  (bind _teamid (Default|GetTeamID _asbp_third_person_character))
  (Development|PrintString (Utilities|String|Append "Name: " (PlayerState|GetPlayerName (Variables|/Script/Engine.Pawn|GetPlayerState _asbp_third_person_character)) " " "TeamID: " _teamid))
  (bind _asbp_third_person_player_controller (Utilities|Casting|CastToBP_ThirdPersonPlayerController (Game|GetPlayerController 0)))
  (Development|PrintString (Utilities|String|Append "Name: " (PlayerState|GetPlayerName (Variables|/Script/Engine.Controller|GetPlayerState _asbp_third_person_player_controller)) " " "TeamID: " (Variables|/Game/Core/GameModes/Game/BP_ThirdPersonPlayerController.BP_ThirdPersonPlayerController_C|GetTeamID _asbp_third_person_player_controller)))
  (return (Utilities|Enum|Equal(Enum) (Variables|/Game/Core/GameModes/Game/BP_ThirdPersonPlayerController.BP_ThirdPersonPlayerController_C|GetTeamID _asbp_third_person_player_controller) _teamid)))