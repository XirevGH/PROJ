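; Gameplay Ability for cast-time projectile abilities, driven by AbilityData and ProjectileData.
; Activation plays start sound, particle and rate-scaled montage, and writes cast info to BP_ThirdPersonCharacter.
; An Event.Cast.Execute gameplay event starts the montage's Cast section; authority alone then commits, plays cast sound and muzzle flash, calls Cast and ends.
; Interrupting the start montage cancels the ability; any cancelled end calls InterruptCast on the character.
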(event Ability|EventActivateAbility
  (bind _projectiledata (Variables|Default|GetProjectileData))
  (bind _abilitydata (Variables|Default|GetAbilityData))
  (bind _abilitydata_2 (Variables|Default|GetAbilityData))
  (bind _projectiledata_2 (Variables|Default|GetProjectileData))
  (bind _abilitydata_3 (Variables|Default|GetAbilityData))
  (bind _abilitysound (Variables|/Script/PROJ.AbilityData|GetAbilitySound _abilitydata_2))
  (bind _abilitysound_2 (Variables|/Script/PROJ.AbilityData|GetAbilitySound _abilitydata))
  (bind _castparticle (Variables|/Script/PROJ.ProjectileDataAsset|GetCastParticle _projectiledata_2))
  (bind _montage (Variables|/Script/PROJ.AbilityData|GetMontage _abilitydata_3))
  (bind _muzzleflashparticle (Variables|/Script/PROJ.ProjectileDataAsset|GetMuzzleFlashParticle _projectiledata))
  (bind _returnvalue (Class|BaseGameplayAbility|CalculateAbilityMontagePlayRate))
  (Utilities|FlowControl|Sequence
    (:then_0
      (Utilities|IsValid _abilitysound_2
        (:Is%20Valid
          (bind _returnvalue_2 (Audio|SpawnSoundatLocation _abilitysound_2 (Transformation|GetActorLocation (Ability|GetAvatarActorfromActorInfo)) "0, 0, 0" 1.0 1.0 0.0 0 0))
          (Class|AudioParameterControllerInterface|SetTriggerParameter _returnvalue_2 "Start"))))
    (:then_1
      (Utilities|IsValid _castparticle
        (:Is%20Valid
          (Effects|SpawnEmitterAttached _castparticle (Class|GameplayAbility|GetOwningComponentfromActorInfo) (Variables|Default|GetSpawnSocketName)))))
    (:then_2
      (|PlayMontageandWaitProxy "None" _montage _returnvalue "Start" false 1.0 0.0 false
        (:then
          (Ability|Tasks|WaitGameplayEvent "(TagName=\"Event.Cast.Execute\")" 0
            (:then
              (CallFunction|SetCastNotify))
            (:EventReceived
              (|PlayMontageandWaitProxy "None" _montage 1.0 "Cast" false 1.0 0.0 false
                (:then
                  (Ability|HasAuthority
                    (:True
                      (Ability|CommitAbility)
                      (Utilities|FlowControl|Sequence
                        (:then_0
                          (Utilities|IsValid _abilitysound
                            (:Is%20Valid
                              (bind _returnvalue_3 (Audio|SpawnSoundatLocation _abilitysound (Transformation|GetActorLocation (Ability|GetAvatarActorfromActorInfo)) "0, 0, 0" 1.0 1.0 0.0 0 0))
                              (Class|AudioParameterControllerInterface|SetTriggerParameter _returnvalue_3 "Cast"))))
                        (:then_1
                          (Utilities|IsValid _muzzleflashparticle
                            (:Is%20Valid
                              (Effects|SpawnEmitterAttached _muzzleflashparticle (Class|GameplayAbility|GetOwningComponentfromActorInfo) (Variables|Default|GetSpawnSocketName)))))
                        (:then_2
                          (Class|GACastProjectile|Cast)
                          (Ability|EndAbility))))))))))
        (:OnCompleted
          (Ability|EndAbility))
        (:OnInterrupted
          (Ability|CancelAbility :!label _label))
        (:OnCancelled
          (goto _label))))))

(event Ability|EventOnEndAbility
  (params (bWasCancelled :type Boolean))
  (if bWasCancelled
    (bind _asbp_third_person_character (Utilities|Casting|CastToBP_ThirdPersonCharacter (Ability|GetAvatarActorfromActorInfo)))
    (Default|InterruptCast _asbp_third_person_character (Variables|Default|GetCastTime))))

(fn SetCastNotify
  (bind _asbp_third_person_character (Utilities|Casting|CastToBP_ThirdPersonCharacter (Ability|GetAvatarActorfromActorInfo)))
  (Variables|/Game/Characters/Base/_Core/BP_ThirdPersonCharacter.BP_ThirdPersonCharacter_C|SetCurrentCastInfo _asbp_third_person_character (Utilities|Struct|MakeS_CastInfo (Variables|Default|GetCastTime) (Variables|Default|GetAbilityName) (.millisecond (Math|DateTime|Now)))))