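; Game instance Blueprint that moves players between EOS lobby and match sessions.
; Joining a lobby (refused when full or matchmaking) or match stores the target session, then destroys the current one with a next-action tag; the destroy-completed callback joins the stored session.
; A found match's custom session name is passed through the player state; non-server players search sessions for that name to follow into the match.
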(event Custom|Event_OnDestroySessionComplete
  (params (bWasSuccessful :type Boolean) (NextAction :type EDestroySessionNextAction%20Enum :default "JoinLobby"))
  (bind _sessiontojoin (Variables|Default|GetSessionToJoin))
  (Development|PrintString "OnDestroySession event")
  (if bWasSuccessful
    (switch Utilities|FlowControl|Switch|SwitchonEDestroySessionNextAction NextAction
      (:JoinLobby
        _)
      (:HostJoinMatch
        _)
      (:ClientJoinMatch
        _))
    (|JoinSession (Game|GetPlayerController 0) _sessiontojoin
      (:OnSuccess
        (bind _extrasettings (Class|AdvancedSessionsLibrary|GetExtraSettings _sessiontojoin))
        (bind _settingvalue (Class|AdvancedSessionsLibrary|GetSessionPropertyString _extrasettings (Utilities|String|StringToName (Class|EOSGameInstance|GetCustomSessionNameKey)))
          (:Found
            (Class|EOSGameInstance|HandleSuccessfulJoin _settingvalue)
            (Development|PrintString "Joined Session"))))
      (:OnFailure
        (Development|PrintString "Failed to join session")))
    (else
      (Development|PrintString "OnDestroySession failed"))))

(event Custom|JoinMatch
  (params (CustomSessionName :type String))
  (Development|PrintString "Join Match")
  (if (Networking|IsServer)
    (Class|EOSGameInstance|DestroyCurrentSession "HostJoinMatch")
    (else
      (bind _results (|FindSessions (Game|GetPlayerController 0) 100 false true)
        (:OnSuccess
          (bind _array_element (Utilities|Array|ForEachLoopwithBreak _results :!label _label)
            (:LoopBody
              (Development|PrintString (Class|FindSessionsCallbackProxy|GetServerName _array_element))
              (bind _extrasettings (Class|AdvancedSessionsLibrary|GetExtraSettings _array_element))
              (bind _settingvalue (Class|AdvancedSessionsLibrary|GetSessionPropertyString _extrasettings (Utilities|String|StringToName (Class|EOSGameInstance|GetCustomSessionNameKey)))
                (:Found
                  (Development|PrintString (Utilities|String|Append "match to find with custom name: " CustomSessionName))
                  (Development|PrintString (Utilities|String|Append "found custom name: " _settingvalue))
                  (Development|PrintString "Lobby member found session with custom name")
                  (Variables|Default|SetSessionToJoin _array_element)
                  (bind _asbp_player_state (Utilities|Casting|CastToBP_PlayerState (Game|GetPlayerState 0))
                    (:then
                      (Default|ROSLobbyMemberJoiningMatch _asbp_player_state)
                      (if (Utilities|Enum|Equal(Enum) _settingvalue CustomSessionName)
                        (Class|EOSGameInstance|DestroyCurrentSession "ClientJoinMatch")
                        (goto _label Break)
                        (else
                          (Development|PrintString "Custom name does not match"))))
                    (:CastFailed
                      (Development|PrintString "failed to cast player state"))))
                (:NotFound
                  (Development|PrintString "CustomSessionNameKey didi not exist"))))))
        (:OnFailure
          (Development|PrintString "Client: Failed to find match sessions"))))))

(event Custom|JoinLobby
  (params (SessionToJoin :type Blueprint%20Session%20Result%20Structure%20%28by%20ref%29))
  (Variables|Default|SetSessionToJoin SessionToJoin)
  (Development|PrintString "JoinLobby")
  (if (< (Class|FindSessionsCallbackProxy|GetCurrentPlayers SessionToJoin) 3)
    (if (Class|EOSGameInstance|GetIsSearchingforMatch)
      (Development|PrintString "Cannot join lobby that searches for match")
      (else
        (Class|EOSGameInstance|DestroyCurrentSession "JoinLobby")))
    (else
      (Development|PrintString "Cannot join full lobby"))))

(event EventOnMatchSessionFound
  (params (FoundMatchSession :type Blueprint%20Session%20Result%20Structure))
  (Variables|Default|SetSessionToJoin FoundMatchSession)
  (bind _asbp_player_state (Utilities|Casting|CastToBP_PlayerState (Game|GetPlayerState 0)))
  (bind _extrasettings (Class|AdvancedSessionsLibrary|GetExtraSettings FoundMatchSession))
  (bind _settingvalue (Class|AdvancedSessionsLibrary|GetSessionPropertyString _extrasettings (Utilities|String|StringToName (Class|EOSGameInstance|GetCustomSessionNameKey)))
    (:Found
      (Default|ClientJoinFoundMatch _asbp_player_state _settingvalue)
      (bind _asbp_lobby_game_mode (Utilities|Casting|CastToBP_LobbyGameMode (Game|GetGameMode)))
      (switch Utilities|FlowControl|Switch|SwitchonE_GameModes (Variables|/Game/Blueprints/Lobby/BP_LobbyGameMode.BP_LobbyGameMode_C|GetSelectedGameMode _asbp_lobby_game_mode)
        (:NewEnumerator0
          (CallFunction|JoinMatch _settingvalue))))
    (:NotFound
      (Development|PrintString "OnMatchFound: Custom session name not found"))))

(event EventInit
  (Development|PrintString "Blueprint game instance init")
  (EventDispatchers|BindEventtoOnDestroySessionCompletedwithNextAction (delegate Custom|Event_OnDestroySessionComplete)))