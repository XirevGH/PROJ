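; Gameplay ability for a player-confirmed, ground-targeted area-of-effect cast with debug prints and sphere.
; It commits, then waits on BP_GroundTrace_Indicator for a target point within Range, ending if cancelled.
; On confirm it spawns BP_SingularitySpike there and sphere-overlaps Pawns within Radius, excluding the caster.
; Each target's own ability system builds and self-applies the first default effect, with BaseDamage set by caller through Data.Damage.
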(event Ability|EventActivateAbility
  (bind _radius (Variables|Default|GetRadius))
  (Ability|CommitAbility)
  (bind _data (|WaitTargetData :ConfirmationType "UserConfirmed" :Class "/Game/Ability_Indicators/BP_GroundTrace_Indicator.BP_GroundTrace_Indicator_C" :MaxRange (Variables|Default|GetRange) :TraceProfile "(Name=\"BlockAll\")" :StartLocation (Class|GameplayAbility|MakeTargetLocationInfofromOwnerActor) :ReticleClass 0)
    (:ValidData
      (Development|PrintString "has target")
      (Development|PrintString (Utilities|GetDisplayName (Utilities|Array|Get(acopy) (Ability|TargetData|GetActorsfromTargetData _data))))
      (bind _outactors (Collision|SphereOverlapActors (Class|AbilitySystemBlueprintLibrary|GetTargetDataEndPoint _data) _radius (Utilities|Array|MakeArray "ObjectTypeQuery2") "/Script/Engine.Pawn" (Utilities|Array|MakeArray (Ability|GetAvatarActorfromActorInfo))))
      (Rendering|Debug|DrawDebugSphere (Class|AbilitySystemBlueprintLibrary|GetTargetDataEndPoint _data) _radius 12 "(R=1.000000,G=0.044036,B=0.000167,A=1.000000)" 1.0)
      (Game|SpawnActorfromClass "/Game/Characters/Singularist/BP_SingularitySpike.BP_SingularitySpike_C" (Math|Conversions|ToTransform(Vector) (Class|AbilitySystemBlueprintLibrary|GetTargetDataEndPoint _data)) "AlwaysSpawn" "MultiplyWithRoot" 0 0)
      (for _array_element _outactors
        (bind _returnvalue (Ability|GameplayEffect|AssignTagSetbyCallerMagnitude (GameplayEffects|MakeOutgoingSpec (Ability|GetAbilitySystemComponent _array_element) (Utilities|Array|Get(acopy) (Variables|Default|GetDefaultEffects)) 0.0 (GameplayEffects|MakeEffectContext (Ability|GetAbilitySystemComponent _array_element))) "(TagName=\"Data.Damage\")" (Variables|Default|GetBaseDamage)))
        (GameplayEffects|ApplyGameplayEffectSpecToSelf (Ability|GetAbilitySystemComponent _array_element) _returnvalue)
        (Development|PrintString "has target")
        (Development|PrintString (Utilities|GetDisplayName _array_element)))
      (Ability|EndAbility))
    (:Cancelled
      (Development|PrintString "cancel")
      (Ability|EndAbility))))