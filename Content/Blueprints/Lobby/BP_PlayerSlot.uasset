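; BP_PlayerSlot is a lobby slot that displays a player's selected character at its Arrow component.
; AddPlayer stores the controller and spawns its BP_LobbyController's SelectedCharacterClass.
; SwitchCharacter shares that spawn path, replacing any existing character and raising the new one by its capsule half-height.
; RemovePlayer clears PlayerController before checking its validity, so its destroy branch never runs and the character remains.
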(event Custom|AddPlayer
  (params (PlayerController :type Player%20Controller%20Object%20Reference))
  (bind _arrow (Variables|Default|GetArrow))
  (bind _returnvalue (Transformation|GetWorldTransform _arrow))
  (bind _output_get (Variables|Default|SetPlayerController PlayerController))
  (bind _asbp_lobby_controller (Utilities|Casting|CastToBP_LobbyController _output_get))
  (Variables|Default|SetCharacterToSpawn (Variables|/Game/Blueprints/Lobby/BP_LobbyController.BP_LobbyController_C|GetSelectedCharacterClass _asbp_lobby_controller))
  (bind _selectedcharacter (Variables|Default|GetSelectedCharacter)
    (:then
      (Actor|DestroyActor _selectedcharacter))
    (:else
      _))
  (bind _returnvalue_2 (Game|SpawnActorfromClass (Variables|Default|GetCharacterToSpawn) (Transformation|GetWorldTransform (Variables|Default|GetArrow)) "AlwaysSpawn" "MultiplyWithRoot" 0 0))
  (bind _output_get_2 (Variables|Default|SetSelectedCharacter _returnvalue_2))
  (Transformation|SetActorTransform _output_get_2 (Math|Transform|MakeTransform (Math|Vector|MakeVector (.x (.location _returnvalue)) (.y (.location _returnvalue)) (+ (Components|Capsule|GetScaledCapsuleHalfHeight (Variables|/Script/Engine.Character|GetCapsuleComponent _returnvalue_2)) (.z (.location _returnvalue)))) (.rotation _returnvalue) (.scale _returnvalue))))

(event Custom|RemovePlayer
  (Variables|Default|SetPlayerController 0)
  (bind _playercontroller (Variables|Default|GetPlayerController)
    (:then
      (Actor|DestroyActor _playercontroller)
      (Variables|Default|SetSelectedCharacter 0))
    (:else)))

(event Custom|SwitchCharacter
  (params (CharacterToSpawn :type BP%20Third%20Person%20Character%20Class%20Reference))
  (bind _arrow (Variables|Default|GetArrow))
  (bind _returnvalue (Transformation|GetWorldTransform _arrow))
  (Variables|Default|SetCharacterToSpawn CharacterToSpawn)
  (bind _selectedcharacter (Variables|Default|GetSelectedCharacter)
    (:then
      (Actor|DestroyActor _selectedcharacter))
    (:else
      _))
  (bind _returnvalue_2 (Game|SpawnActorfromClass (Variables|Default|GetCharacterToSpawn) (Transformation|GetWorldTransform (Variables|Default|GetArrow)) "AlwaysSpawn" "MultiplyWithRoot" 0 0))
  (bind _output_get (Variables|Default|SetSelectedCharacter _returnvalue_2))
  (Transformation|SetActorTransform _output_get (Math|Transform|MakeTransform (Math|Vector|MakeVector (.x (.location _returnvalue)) (.y (.location _returnvalue)) (+ (Components|Capsule|GetScaledCapsuleHalfHeight (Variables|/Script/Engine.Character|GetCapsuleComponent _returnvalue_2)) (.z (.location _returnvalue)))) (.rotation _returnvalue) (.scale _returnvalue))))

(fn ConstructionScript)