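; BP_LobbyController is the lobby player controller that shows the lobby menu and passes player choices to their player state.
; On BeginPlay, the local controller creates WBP_LobbyUI, shows the cursor and switches to UI-only input.
; Server_ events write ready state, character class and nameplate name to BP_PlayerState.
; A ready change also has BP_LobbyGameMode check whether all players are ready.
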(event Custom|Server_SetPlayerReady
  (params (bIsReady :type Boolean))
  (bind _asbp_player_state (Utilities|Casting|CastToBP_PlayerState (Variables|GetPlayerState)))
  (Variables|/Game/Core/Game/BP_PlayerState.BP_PlayerState_C|SetbLobby_IsPlayerReady _asbp_player_state bIsReady)
  (bind _asbp_lobby_game_mode (Utilities|Casting|CastToBP_LobbyGameMode (Game|GetGameMode)))
  (Default|CheckAllPlayersReady _asbp_lobby_game_mode))

(event Custom|Server_SwitcCharacterClass
  (params (CharacterClass :type BP%20Third%20Person%20Character%20Class%20Reference))
  (bind _asbp_player_state (Utilities|Casting|CastToBP_PlayerState (Variables|GetPlayerState)))
  (Variables|/Game/Core/Game/BP_PlayerState.BP_PlayerState_C|SetCharacterClass _asbp_player_state CharacterClass))

(event Custom|Server_UpdatePlayerInfoName
  (bind _asbp_player_state (Utilities|Casting|CastToBP_PlayerState (Variables|GetPlayerState)))
  (Variables|/Game/Core/Game/BP_PlayerState.BP_PlayerState_C|SetPlayerNameplateName _asbp_player_state (Class|AdvancedSessionsLibrary|GetPlayerName self)))

(event EventBeginPlay
  (if (Pawn|IsLocalPlayerController)
    (bind _returnvalue (UserInterface|CreateWidget "/Game/UI/Lobby/WBP_LobbyUI.WBP_LobbyUI_C"))
    (bind _output_get (Variables|Default|SetLobby%20UI _returnvalue))
    (UserInterface|Viewport|AddtoViewport _output_get 0)
    (Variables|Default|SetbShowMouseCursor true)
    (Input|SetInputModeUIOnly self (Variables|Default|GetLobby%20UI) "DoNotLock" false)))

(fn ConstructionScript)