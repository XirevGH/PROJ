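; Lobby game mode that manages party players, ready state and the handoff into team matches.
; Joins and logouts update tag-indexed player slots, after a delay-loop wait for slot setup, and shrink or restore available game modes by party size.
; While matchmaking, it either counts joining opponents before server-travelling to the match level, or counts departed party members before the host joins the match session, using thresholds from the selected mode.
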(event Custom|ROS_TravelToMatchLevel
  (bind _asbp_game_instance (Utilities|Casting|CastToBP_GameInstance (Game|GetGameInstance)))
  (Class|AdvancedGameInstance|SetIsSearchingforMatch _asbp_game_instance false)
  (Class|AdvancedSessionsLibrary|ServerTravel (Variables|Default|GetMatchLevelURL) false false)
  (Development|PrintString "Travel to match executed on server"))

(event Custom|ROS_OnLobbyMemberJoiningMatch
  (bind _result (Math|Integer|IncrementInt (Variables|Default|GetLobbyMembersJoinedMatch))
    (:%20%20
      (Variables|Default|SetLobbyMembersJoinedMatch _result)
      (Development|PrintString "Lobby member left and joined match session")
      (Development|PrintString (Utilities|String|Append "Members who have left: " (Utilities|String|ToString(Integer) (Variables|Default|GetLobbyMembersJoinedMatch)))))))

(event EventBeginPlay
  (CallFunction|SetPlayerSlots)
  (for _array_element (Variables|Default|GetAllGameModes)
    (Utilities|Array|Add (Variables|Default|GetAvailableGameModes) _array_element)))

(event EventPostLogin
  (params (NewPlayer :type Player%20Controller%20Object%20Reference))
  (bind _availablegamemodes (Variables|Default|GetAvailableGameModes))
  (bind _playercontrollers (Variables|Default|GetPlayerControllers))
  (bind _asbp_game_instance (Utilities|Casting|CastToBP_GameInstance (Game|GetGameInstance)))
  (if (Class|AdvancedGameInstance|GetIsSearchingforMatch _asbp_game_instance)
    (CallFunction|HandleJoiningOpponents)
    (else
      (bind _asbp_lobby_controller (Utilities|Casting|CastToBP_LobbyController NewPlayer))
      (Variables|/Game/Blueprints/Lobby/BP_LobbyController.BP_LobbyController_C|SetTeamID _asbp_lobby_controller (Class|AdvancedSessionsLibrary|UniqueNetIdtoString (Class|AdvancedSessionsLibrary|GetUniqueNetID (Game|GetPlayerController 0))))
      (Utilities|Array|Add _playercontrollers NewPlayer)
      (if (> (Utilities|Array|Length _playercontrollers) 1)
        (Utilities|Array|RemoveIndex _availablegamemodes (Utilities|Array|LastIndex _availablegamemodes)))
      (Utilities|IfPlayerSlotsSet
        (:true
          (CallFunction|UpdatePlayerSlots)
          (bind _asbp_lobby_controller_2 (Utilities|Casting|CastToBP_LobbyController (Game|GetPlayerController 0)))
          (Utilities|IsValid (Variables|/Game/Blueprints/Lobby/BP_LobbyController.BP_LobbyController_C|GetLobby%20UI _asbp_lobby_controller_2)
            (:Is%20Valid
              (Default|UpdateAvailableGameModes (Variables|/Game/Blueprints/Lobby/BP_LobbyController.BP_LobbyController_C|GetLobby%20UI _asbp_lobby_controller_2)))))))))

(event EventOnLogout
  (params (ExitingController :type Controller%20Object%20Reference))
  (bind _playercontrollers (Variables|Default|GetPlayerControllers))
  (bind _asbp_game_instance (Utilities|Casting|CastToBP_GameInstance (Game|GetGameInstance)))
  (if (Class|AdvancedGameInstance|GetIsSearchingforMatch _asbp_game_instance)
    (CallFunction|CheckforHosttoJoinMatch))
  (bind _asplayer_controller (Utilities|Casting|CastToPlayerController ExitingController))
  (if (Utilities|Array|ContainsItem (Variables|Default|GetPlayerControllers) _asplayer_controller)
    (Utilities|Array|RemoveItem _playercontrollers _asplayer_controller)
    (if (> (Utilities|Array|Length _playercontrollers) 1)
      (CallFunction|ReAddGameModeonLogout))
    (Utilities|IfPlayerSlotsSet
      (:true
        (CallFunction|UpdatePlayerSlots)
        (bind _asbp_lobby_controller (Utilities|Casting|CastToBP_LobbyController (Game|GetPlayerController 0)))
        (Utilities|IsValid (Variables|/Game/Blueprints/Lobby/BP_LobbyController.BP_LobbyController_C|GetLobby%20UI _asbp_lobby_controller)
          (:Is%20Valid
            (Default|UpdateAvailableGameModes (Variables|/Game/Blueprints/Lobby/BP_LobbyController.BP_LobbyController_C|GetLobby%20UI _asbp_lobby_controller))))))))

(fn ConstructionScript)

(fn SetPlayerSlots
  (bind _outactors (Actor|GetAllActorsOfClass "/Game/Blueprints/Lobby/BP_PlayerSlot.BP_PlayerSlot_C"))
  (for _index (range 0 (Utilities|Array|LastIndex _outactors))
    (bind _outactors_2 (Actor|GetAllActorsOfClasswithTag "/Game/Blueprints/Lobby/BP_PlayerSlot.BP_PlayerSlot_C" (Utilities|String|StringToName (Utilities|String|ToString(Integer) _index))))
    (Utilities|Array|Add (Variables|Default|GetPlayer%20Slots) (Utilities|Array|Get(acopy) _outactors_2)))
  (Variables|Default|SetSetSlotsDone true))

(fn UpdatePlayerSlots
  ;[0.15 0.15 0.15 0.5] Check if player controller is already added
  (for _array_element (Variables|Default|GetPlayerControllers)
    (LocalVariables|SetPlayerControllerAlreadyAdded false)
    (bind _array_element_2 (Utilities|Array|ForEachLoopwithBreak (Variables|Default|GetPlayer%20Slots) :!label _label)
      (:LoopBody
        (if (== (Variables|/Game/Blueprints/Lobby/BP_PlayerSlot.BP_PlayerSlot_C|GetPlayerController _array_element_2) _array_element)
          (LocalVariables|SetPlayerControllerAlreadyAdded true)
          (goto _label Break)))
      (:Completed
        ;[0.15 0.15 0.15 0.5] Add player controller to player slot
        (if (not (LocalVariables|GetPlayerControllerAlreadyAdded))
          (bind _array_element_3 (Utilities|Array|ForEachLoopwithBreak (Variables|Default|GetPlayer%20Slots) :!label _label_2)
            (:LoopBody
              (Variables|/Game/Blueprints/Lobby/BP_PlayerSlot.BP_PlayerSlot_C|GetPlayerController _array_element_3
                (:then)
                (:else
                  (Default|AddPlayer _array_element_3 _array_element)
                  (goto _label_2 Break)))))))))
  (for _array_element_4 (Variables|Default|GetPlayer%20Slots)
    (if (not (Utilities|Array|ContainsItem (Variables|Default|GetPlayerControllers) (Variables|/Game/Blueprints/Lobby/BP_PlayerSlot.BP_PlayerSlot_C|GetPlayerController _array_element_4)))
      (Default|RemovePlayer _array_element_4))))

(fn UpdatePlayerInfo
  (params (RequestingPlayerController :type Player%20Controller%20Object%20Reference))
  (bind _array_element (Utilities|Array|ForEachLoopwithBreak (Variables|Default|GetPlayer%20Slots))
    (:LoopBody
      (if (== (Variables|/Game/Blueprints/Lobby/BP_PlayerSlot.BP_PlayerSlot_C|GetPlayerController _array_element) RequestingPlayerController)
        (Utilities|Casting|CastToBP_LobbyController RequestingPlayerController)
        (if (== (Utilities|GetClass (Variables|/Game/Blueprints/Lobby/BP_PlayerSlot.BP_PlayerSlot_C|GetSelectedCharacter _array_element)) 0)
          (Utilities|Casting|CastToBP_LobbyController RequestingPlayerController)
          (bind _asbp_player_state (Utilities|Casting|CastToBP_PlayerState (Variables|/Script/Engine.Controller|GetPlayerState RequestingPlayerController))))))
    (:Completed
      (Utilities|Casting|CastToBP_LobbyController RequestingPlayerController))))

(fn CheckAllPlayersReady
  (LocalVariables|SetAllPlayersReady true)
  (for _array_element (Variables|Default|GetPlayerControllers)
    (bind _asbp_player_state (Utilities|Casting|CastToBP_PlayerState (Variables|/Script/Engine.Controller|GetPlayerState _array_element))
      (:then
        (if (not (Variables|/Game/Core/Game/BP_PlayerState.BP_PlayerState_C|GetbLobby_IsPlayerReady _asbp_player_state))
          (LocalVariables|SetAllPlayersReady false)))
      (:CastFailed
        (Development|PrintString "player state cast failed"))))
  (bind _asbp_lobby_controller (Utilities|Casting|CastToBP_LobbyController (Game|GetPlayerController 0)))
  (Variables|/Game/UI/Lobby/WBP_LobbyUI.WBP_LobbyUI_C|SetAllPlayerReady (Variables|/Game/Blueprints/Lobby/BP_LobbyController.BP_LobbyController_C|GetLobby%20UI _asbp_lobby_controller) (LocalVariables|GetAllPlayersReady)))

(fn OnRepSelectedGameMode)

(fn ReAddGameModeonLogout
  (bind _arrayelement (Utilities|Array|ReverseforEachLoop (Variables|Default|GetAllGameModes))
    (:LoopBody
      (if (not (Utilities|Array|ContainsItem (Variables|Default|GetAvailableGameModes) _arrayelement))
        (Utilities|Array|Add (Variables|Default|GetAvailableGameModes) _arrayelement)
        (return)))))

(fn PlayingSolo
  (return (== (Utilities|Array|Length (Variables|Default|GetAllGameModes)) (Utilities|Array|Length (Variables|Default|GetAvailableGameModes)))))

(fn HandleJoiningOpponents
  (Development|PrintString (Utilities|String|Append "Player who called HandleJoiningOpoenents " (Class|AdvancedSessionsLibrary|GetPlayerName (Game|GetPlayerController 0))))
  (bind _result (Math|Integer|IncrementInt (Variables|Default|GetMatchOponentsJoined))
    (:%20%20
      (Variables|Default|SetMatchOponentsJoined _result)
      (switch Utilities|FlowControl|Switch|SwitchonE_GameModes (Variables|Default|GetSelectedGameMode)
        (:NewEnumerator0
          (if (== (Variables|Default|GetMatchOponentsJoined) 1)
            (Development|PrintString "All oponents have joined" :!label _label)
            (CallFunction|ROSTraveltoMatchLevel)))
        (:NewEnumerator1
          (if (== (Variables|Default|GetMatchOponentsJoined) 2)
            (goto _label)))
        (:NewEnumerator2
          (if (== (Variables|Default|GetMatchOponentsJoined) 3)
            (goto _label)))))))

(fn CheckforHosttoJoinMatch
  (switch Utilities|FlowControl|Switch|SwitchonE_GameModes (Variables|Default|GetSelectedGameMode)
    (:NewEnumerator1
      (if (== (Variables|Default|GetLobbyMembersJoinedMatch) 1)
        (Development|PrintString "All members have joined the match" :!label _label)
        (bind _asbp_game_instance (Utilities|Casting|CastToBP_GameInstance (Game|GetGameInstance)))
        (Default|JoinMatch _asbp_game_instance)))
    (:NewEnumerator2
      (if (== (Variables|Default|GetLobbyMembersJoinedMatch) 2)
        (goto _label)))))