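; Base game mode that tracks connected third-person player controllers and links each one to its player state.
; Post-login and controller swaps wait two seconds, then call SetPlayerNameplate, which adds the controller to AllPlayers and stores it on its BP_PlayerState.
; Logout removes the controller from the list.
; Despite the function's name, no nameplate is set: the character-created binding and name lookup are disconnected, and GetCharacter is empty.
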(event EventOnLogout
  (params (ExitingController :type Controller%20Object%20Reference))
  (bind _asbp_third_person_player_controller (Utilities|Casting|CastToBP_ThirdPersonPlayerController ExitingController))
  (Utilities|Array|RemoveItem (Variables|Default|GetAll_Players) _asbp_third_person_player_controller))

(event EventPostLogin
  (params (NewPlayer :type Player%20Controller%20Object%20Reference))
  (Utilities|FlowControl|Delay 2.0)
  (bind _output_get (Variables|Default|Setbool true))
  (CallFunction|SetPlayerNameplate NewPlayer _output_get))

(event EventOnSwapPlayerControllers
  (params (OldPC :type Player%20Controller%20Object%20Reference) (NewPC :type Player%20Controller%20Object%20Reference))
  (Utilities|FlowControl|Delay 2.0)
  (bind _output_get (Variables|Default|Setbool false))
  (CallFunction|SetPlayerNameplate NewPC _output_get))

(fn ConstructionScript)

(fn SetPlayerNameplate
  (params (PlayerController :type Player%20Controller%20Object%20Reference) (onlogin :type Boolean))
  (if onlogin
    (Development|PrintString "PostLogin")
    (else
      (Development|PrintString "SwapController")))
  (bind _asbp_third_person_player_controller (Utilities|Casting|CastToBP_ThirdPersonPlayerController PlayerController))
  (Utilities|Array|Add (Variables|Default|GetAll_Players) _asbp_third_person_player_controller)
  (bind _asbp_player_state (Utilities|Casting|CastToBP_PlayerState (Variables|/Script/Engine.Controller|GetPlayerState _asbp_third_person_player_controller)))
  (Variables|/Game/Core/Game/BP_PlayerState.BP_PlayerState_C|SetPlayerController _asbp_player_state _asbp_third_person_player_controller))

(fn GetCharacter)