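; Character Blueprint for the Singularist, which so far only adds a debug hook for ability cooldown tag changes.
; On BeginPlay it runs the parent logic, then binds an event wrapper to the Cooldown.Ability gameplay tag on the Ability System Component obtained from PlayerState.
; The bound event prints a placeholder "Hello" and ignores the tag and count.
; The construction script only calls the parent.
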(event Custom|CustomEvent
  (params (Tag :type Gameplay%20Tag%20Structure%20%28by%20ref%29) (TagCount :type Integer))
  (Development|PrintString "Hello"))

(event EventBeginPlay
  (|CallParentFunction)
  (Class|AbilitySystemBlueprintLibrary|BindEventWrappertoAnyOfGameplayTagsChanged (Ability|GetAbilitySystemComponent (Variables|Default|GetPlayerState self)) (Utilities|Array|MakeArray "(TagName=\"Cooldown.Ability\")") (delegate Custom|CustomEvent)))

(event Collision|EventActorBeginOverlap
  (params (OtherActor :type Actor%20Object%20Reference)))

(event EventTick
  (params (DeltaSeconds :type Float%20%28single-precision%29)))

(fn ConstructionScript
  (|CallParentFunction))