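; Projectile for the Singularist's secondary ability that becomes a short-lived gravity well, pulling characters other than the caster toward its center.
; Its Sphere starts with collision disabled; a valid hit or overlap stops the projectile, enables the Sphere for queries and starts a timed self-destroy.
; Tick drags overlapping characters inward at constant speed with swept SetActorLocation calls rather than physics forces.
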(event Custom|CustomEvent
  (Actor|DestroyActor))

(event EventBeginPlay
  (|CallParentFunction)
  (Collision|SetCollisionEnabled (Variables|Default|GetSphere) "NoCollision"))

(event EventTick
  (params (DeltaSeconds :type Float%20%28single-precision%29))
  (|CallParentFunction DeltaSeconds)
  (for _array_element (Collision|GetOverlappingActors (Variables|Default|GetSphere) "/Script/Engine.Character" :!class /Script/Engine.PrimitiveComponent)
    (if (not (== (Variables|Default|GetCaster) _array_element))
      (bind _ascharacter (Utilities|Casting|CastToCharacter _array_element))
      (if (not (Utilities|Operators|EqualEqual (Transformation|GetActorLocation) (Transformation|GetActorLocation _ascharacter) 0.2))
        (Transformation|SetActorLocation _ascharacter (Math|Interpolation|VInterptoConstant (Transformation|GetActorLocation _ascharacter) (Transformation|GetActorLocation) DeltaSeconds 5e+02) true false)))))

(event EventOnProjectileHit
  (params (HitComp :type Primitive%20Component%20Object%20Reference) (OtherActor :type Actor%20Object%20Reference) (OtherComp :type Primitive%20Component%20Object%20Reference) (NormalImpulse :type Vector :default "0, 0, 0") (Hit :type Hit%20Result%20Structure%20%28by%20ref%29))
  (|CallParentFunction HitComp OtherActor OtherComp NormalImpulse Hit)
  (bind _returnvalue (Class|Projectile|ShouldSkipHit OtherActor))
  (if (not _returnvalue)
    (Variables|/Script/Engine.MovementComponent|SetVelocity (Variables|Default|GetProjectileMovement) "0, 0, 0")
    (Collision|SetCollisionEnabled (Variables|Default|GetSphere) "QueryOnly")
    (Utilities|Time|SetTimerbyEvent (delegate Custom|CustomEvent) 2.0)))

(event EventOnBeginOverlap
  (params (OverlappedComponent :type Primitive%20Component%20Object%20Reference) (OtherActor :type Actor%20Object%20Reference) (OtherComp :type Primitive%20Component%20Object%20Reference) (OtherBodyIndex :type Integer) (bFromSweep :type Boolean) (SweepResult :type Hit%20Result%20Structure%20%28by%20ref%29))
  (|CallParentFunction OverlappedComponent OtherActor OtherComp OtherBodyIndex bFromSweep SweepResult)
  (bind _returnvalue (Class|Projectile|ShouldSkipHit OtherActor))
  (if (not _returnvalue)
    (Variables|/Script/Engine.MovementComponent|SetVelocity (Variables|Default|GetProjectileMovement) "0, 0, 0")
    (Collision|SetCollisionEnabled (Variables|Default|GetSphere) "QueryOnly")
    (Utilities|Time|SetTimerbyEvent (delegate Custom|CustomEvent) 2.0)))

(fn ConstructionScript
  (|CallParentFunction))