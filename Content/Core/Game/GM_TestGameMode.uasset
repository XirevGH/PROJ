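; GM_TestGameMode is a test game mode that gives each joining player a nameplate name taken from their Steam profile.
; On PostLogin it casts the player's state to BP_PlayerState, looks up the Steam persona name from the player's unique net ID, stores it as PlayerNameplateName and prints it.
; BeginPlay and Tick are empty, and a disconnected chain for game-only input mode never runs.
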(event EventBeginPlay)

(event EventTick
  (params (DeltaSeconds :type Float%20%28single-precision%29)))

(event EventPostLogin
  (params (NewPlayer :type Player%20Controller%20Object%20Reference))
  (bind _asbp_player_state (Utilities|Casting|CastToBP_PlayerState (Variables|/Script/Engine.Controller|GetPlayerState NewPlayer))
    (:then
      _)
    (:CastFailed
      (Development|PrintString "Failed cast")))
  (bind _returnvalue (Class|AdvancedSteamFriendsLibrary|GetSteamPersonaName (Class|AdvancedSessionsLibrary|GetUniqueNetID NewPlayer)))
  (bind _output_get (Variables|/Game/Core/Game/BP_PlayerState.BP_PlayerState_C|SetPlayerNameplateName _asbp_player_state _returnvalue))
  (Development|PrintString _output_get))

(fn ConstructionScript)