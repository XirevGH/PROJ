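; Player state that carries each player's lobby ready status, selected class, mannequin and nameplate names, keeping their displays in sync through RepNotifies.
; Lobby changes update the mannequin's player info widget, while a class change asks the mannequin to update its character display.
; When the mannequin replicates, it refreshes that widget and has the lobby controller send name and ready updates to the server.
; The in-game name is printed and written to the third-person pawn's nameplate.
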(event Custom|PlayerName)

(event EventBeginPlay)

(event EventTick
  (params (DeltaSeconds :type Float%20%28single-precision%29)))

(fn ConstructionScript)

(fn OnRepBLobbyIsPlayerReady
  (CallFunction|LobbyUpdateIsReady))

(fn LobbyUpdateIsReady
  (bind _aswbp_player_info (Utilities|Casting|CastToWBP_PlayerInfo (UserInterface|GetUserWidgetObject (Variables|/Game/Blueprints/Lobby/BP_LobbyMannequin.BP_LobbyMannequin_C|GetWidget_Lobby_PlayerInfo (Variables|Default|GetLobby_Mannequin)))))
  (Default|UpdatePlayerReady _aswbp_player_info (Variables|Default|GetbLobby_IsPlayerReady)))

(fn LobbyUpdatePlayerInfoName
  (bind _aswbp_player_info (Utilities|Casting|CastToWBP_PlayerInfo (UserInterface|GetWidget (Variables|/Game/Blueprints/Lobby/BP_LobbyMannequin.BP_LobbyMannequin_C|GetWidget_Lobby_PlayerInfo (Variables|Default|GetLobby_Mannequin)))))
  (Default|SetPlayerNameText _aswbp_player_info (Variables|Default|GetLobby_PlayerNameplateName)))

(fn OnRepSelectedClass
  (Default|ServerUpdateCharacterDisplay (Variables|Default|GetLobby_Mannequin) (Variables|Default|GetSelectedClass)))

(fn OnRepLobbyMannequin
  (CallFunction|LobbyUpdateIsReady)
  (CallFunction|LobbyUpdatePlayerInfoName)
  (bind _asbp_lobby_controller (Utilities|Casting|CastToBP_LobbyController (Game|GetPlayerController)))
  (Default|ServerUpdatePlayerInfoName _asbp_lobby_controller)
  (Default|ServerSetPlayerReady _asbp_lobby_controller (Variables|Default|GetbLobby_IsPlayerReady)))

(fn GameUpdatePlayerNameplate
  (bind _game_playernameplatename (Variables|Default|GetGame_PlayerNameplateName))
  (bind _asbp_third_person_character (Utilities|Casting|CastToBP_ThirdPersonCharacter (PlayerState|GetPawn)))
  (Development|PrintString _game_playernameplatename)
  (Rendering|Components|TextRender|SetText (Variables|/Game/UI/WBP_WidgetNameplate.WBP_WidgetNameplate_C|GetPlayerName (Variables|/Game/ThirdPerson/Blueprints/BP_ThirdPersonCharacter.BP_ThirdPersonCharacter_C|GetNamePlateWidget _asbp_third_person_character)) (Utilities|Text|ToText(String) _game_playernameplatename)))

(fn OnRepGamePlayerNameplateName
  (CallFunction|GameUpdatePlayerNameplate))

(fn OnRepLobbyPlayerNameplateName
  (CallFunction|LobbyUpdatePlayerInfoName))