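; Steam game instance that hosts and joins lobby sessions and moves players from a lobby into a found match.
; CreateSession opens a listen lobby tagged with mode, searching flag and custom name; invites join via JoinLobby after capacity and searching checks.
; A found match's custom name goes to the player state and, in 1v1, JoinMatch.
; The server joins directly; clients search sessions by name, but their compare-and-join branch is disconnected.
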(event Custom|Create%20Session
  (|AdvancedSession (Utilities|Array|MakeArray (Class|AdvancedSessionsLibrary|MakeLiteralSessionPropertyBool (Utilities|String|StringToName (Variables|Default|GetIsSearchingForMatchKey)) false) (Class|AdvancedSessionsLibrary|MakeLiteralSessionPropertyString (Utilities|String|StringToName (Variables|Default|GetSelectedGameModeKey)) "1v1") (Class|AdvancedSessionsLibrary|MakeLiteralSessionPropertyString (Utilities|String|StringToName (Variables|Default|GetCustomSessionNameKey)) (Class|AdvancedSessionsLibrary|GetPlayerName (Game|GetPlayerController 0)))) (Game|GetPlayerController 0) 6 0 false true false true true false false false true false true
    (:OnSuccess
      (Development|PrintString "Created advanced session")
      (Variables|Default|SetbIsTeamLeader true)
      (Game|OpenLevel(byObjectReference) "/Game/Levels/Lvl_Lobby.Lvl_Lobby" true "listen"))))

(event Custom|JoinMatch
  (params (CustomSessionName :type String))
  (Development|PrintString "Join Match")
  (if (Networking|IsServer)
    (|DestroySession (Game|GetPlayerController 0)
      (:OnSuccess
        (|JoinSession (Game|GetPlayerController 0) (Variables|Default|GetMatchToJoin)
          (:OnSuccess
            (Development|PrintString "Team leader joinede match"))
          (:OnFailure
            (Development|PrintString "Team leader failed to join match")))))
    (else
      (bind _results (|FindSessionsAdvanced (Game|GetPlayerController 0) 10 false "AllServers" 0 false false false)
        (:OnSuccess
          (bind _array_element (Utilities|Array|ForEachLoopwithBreak _results)
            (:LoopBody
              (Development|PrintString (Class|FindSessionsCallbackProxy|GetServerName _array_element))
              (bind _extrasettings (Class|AdvancedSessionsLibrary|GetExtraSettings _array_element))
              (bind _settingvalue (Class|AdvancedSessionsLibrary|GetSessionPropertyString _extrasettings (Utilities|String|StringToName (Variables|Default|GetCustomSessionNameKey)))
                (:Found
                  (Development|PrintString (Utilities|String|Append "match to find with custom name: " CustomSessionName))
                  (Development|PrintString (Utilities|String|Append "found custom name: " _settingvalue))
                  (Development|PrintString "Lobby member found session with custom name")
                  (Utilities|Casting|CastToBP_PlayerState (Game|GetPlayerState 0)
                    (:CastFailed
                      (Development|PrintString "failed to cast player state"))))
                (:NotFound
                  (Development|PrintString "CustomSessionNameKey didi not exist"))))))
        (:OnFailure
          (Development|PrintString "Client: Failed to find match sessions"))))))

(event Custom|JoinLobby
  (params (SessionToJoin :type Blueprint%20Session%20Result%20Structure%20%28by%20ref%29))
  (if (< (Class|FindSessionsCallbackProxy|GetCurrentPlayers SessionToJoin) 3)
    (if (Class|AdvancedGameInstance|GetIsSearchingforMatch)
      (Development|PrintString "Cannot join lobby that searches for match")
      (else
        (|DestroySession (Game|GetPlayerController 0)
          (:OnSuccess
            (|JoinSession (Game|GetPlayerController 0) SessionToJoin
              (:OnSuccess
                (Variables|Default|SetbIsTeamLeader false)
                (Development|PrintString (Utilities|String|Append "My Unique ID: " (Class|AdvancedSessionsLibrary|UniqueNetIdtoString (Class|AdvancedSessionsLibrary|GetUniqueNetID (Game|GetPlayerController 0)))))
                (Development|PrintString (Utilities|String|Append "Team Unique ID:  " (Variables|Default|GetUniqueTeamID)))))))))
    (else
      (Development|PrintString "Cannot join full lobby"))))

(event Custom|ROS_MatchFound
  (params (FoundMatchSession :type Blueprint%20Session%20Result%20Structure))
  (Variables|Default|SetMatchToJoin FoundMatchSession)
  (bind _asbp_player_state (Utilities|Casting|CastToBP_PlayerState (Game|GetPlayerState 0)))
  (bind _extrasettings (Class|AdvancedSessionsLibrary|GetExtraSettings FoundMatchSession))
  (bind _settingvalue (Class|AdvancedSessionsLibrary|GetSessionPropertyString _extrasettings (Utilities|String|StringToName (Variables|Default|GetCustomSessionNameKey)))
    (:Found
      (Default|ClientJoinFoundMatch _asbp_player_state _settingvalue)
      (bind _asbp_lobby_game_mode (Utilities|Casting|CastToBP_LobbyGameMode (Game|GetGameMode)))
      (switch Utilities|FlowControl|Switch|SwitchonE_GameModes (Variables|/Game/Core/GameModes/Lobby/BP_LobbyGameMode.BP_LobbyGameMode_C|GetSelectedGameMode _asbp_lobby_game_mode)
        (:NewEnumerator0
          (CallFunction|JoinMatch _settingvalue))))
    (:NotFound
      (Development|PrintString "ROS_MatchFoundDid not find custom name"))))

(event EventOnSessionInviteAccepted
  (params (LocalPlayerNum :type Integer) (PersonInvited :type BP%20Unique%20Net%20Id%20Structure) (SessionToJoin :type Blueprint%20Session%20Result%20Structure%20%28by%20ref%29))
  (CallFunction|JoinLobby SessionToJoin))

(event EventOnMatchSessionFound
  (params (FoundMatchSession :type Blueprint%20Session%20Result%20Structure))
  (CallFunction|ROSMatchFound FoundMatchSession))