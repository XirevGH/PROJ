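; EOS game instance that moves players from a lobby session into a found match session.
; When a match is found, 1v1 calls JoinMatch directly, while 2v2 and 3v3 route the session name through player state 0's ClientJoinFoundMatch.
; JoinMatch has the server join the cached session immediately, while clients first find it by name.
; Both paths show a persistent loading screen, set match join intent and destroy the current session before joining.
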(event Custom|SessionFoundByName
  (params (bWasSuccessful :type Boolean))
  (Development|PrintString "SessionFoundByName called")
  (if bWasSuccessful
    (Development|PrintString "FindSessionByName succeeded")
    (Class|EOSGameInstance|SetClientIsTransitioning true)
    (Class|EOSGameInstance|ShowPersistentLoadingScreen)
    (Class|EOSGameInstance|SetJoinIntent (Class|EOSGameInstance|GetJoinIntentMatch))
    (Class|EOSGameInstance|DestroyCurrentSessionandJoinCachedSession)
    (else
      (Development|PrintString "FindSessionByName failed"))))

(event Custom|JoinMatch
  (params (SessionName :type String))
  (Development|PrintString "Join Match")
  (if (Networking|IsServer)
    (Class|EOSGameInstance|ShowPersistentLoadingScreen)
    (Class|EOSGameInstance|SetJoinIntent (Class|EOSGameInstance|GetJoinIntentMatch))
    (Class|EOSGameInstance|DestroyCurrentSessionandJoinCachedSession)
    (else
      (Class|EOSGameInstance|FindSessionbyName SessionName))))

(event EventOnMatchSessionFound
  (params (Name :type Name :default "None"))
  (bind _returnvalue (Utilities|String|ToString(Name) Name))
  (Class|EOSGameInstance|SetSessionState "JoiningMatch")
  (bind _asbp_lobby_game_mode (Utilities|Casting|CastToBP_LobbyGameMode (Game|GetGameMode)))
  (switch Utilities|FlowControl|Switch|SwitchonE_GameModes (Variables|/Game/Core/GameModes/Lobby/BP_LobbyGameMode.BP_LobbyGameMode_C|GetSelectedGameMode _asbp_lobby_game_mode)
    (:NewEnumerator0
      (CallFunction|JoinMatch _returnvalue))
    (:NewEnumerator1
      (bind _asbp_player_state (Utilities|Casting|CastToBP_PlayerState (Game|GetPlayerState 0) :!label _label))
      (Default|ClientJoinFoundMatch _asbp_player_state _returnvalue))
    (:NewEnumerator2
      (goto _label))))

(event EventInit
  (EventDispatchers|BindEventtoOnSessionFoundbyName (delegate Custom|SessionFoundByName)))