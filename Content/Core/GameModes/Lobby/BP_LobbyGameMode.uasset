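; Lobby game mode that manages party members, matchmaking handoff and return from matches, driven by the EOS game instance's session state.
; Login, logout and controller swaps update controllers, tagged player slots, team size and the game modes available for that party size.
; Join and leave counters trigger either the host's JoinMatch or server travel to the match level, including for Play Again.
; A timer stops loading screens if returning members fail to rejoin.
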(event Custom|ROS_TravelToMatchLevel
  (Development|PrintString "TravelToMatchLevel")
  (Class|AdvancedSessionsLibrary|ServerTravel (Variables|Default|GetMatchLevelURL) false false))

(event Custom|OnAllPlayersFailedToReturn
  (for _array_element (Variables|Default|GetPlayerControllers)
    (bind _asbp_lobby_controller (Utilities|Casting|CastToBP_LobbyController _array_element))
    (Default|ClientStopLoadingScreen _asbp_lobby_controller))
  (Utilities|Time|ClearandInvalidateTimerbyHandle (Variables|Default|GetReturnToLobbyMemberJoinFail))
  (bind _asbp_game_instance_eos (Utilities|Casting|CastToBP_GameInstanceEOS (Game|GetGameInstance)))
  (Class|EOSGameInstance|SetCurrentTeamSize _asbp_game_instance_eos (Utilities|Array|Length (Variables|Default|GetPlayerControllers)))
  (Class|EOSGameInstance|SetSessionState _asbp_game_instance_eos "Lobby"))

(event EventBeginPlay
  (Utilities|FlowControl|Sequence
    (:then_0
      (CallFunction|SetPlayerSlots)
      (for _array_element (Variables|Default|GetAllGameModes)
        (Utilities|Array|Add (Variables|Default|GetAvailableGameModes) (Utilities|Enum|ByteToEnumE_GameModes _array_element))))
    (:then_1
      (bind _asbp_game_instance_eos (Utilities|Casting|CastToBP_GameInstanceEOS (Game|GetGameInstance)))
      (if (Utilities|Enum|Equal(Enum) (Class|EOSGameInstance|GetSessionState _asbp_game_instance_eos) "ReturningToLobbyFromMatch")
        (bind _returnvalue (Utilities|Time|SetTimerbyEvent (delegate Custom|OnAllPlayersFailedToReturn) 25.0))
        (Variables|Default|SetReturnToLobbyMemberJoinFail _returnvalue)))))

(event EventOnSwapPlayerControllers
  (params (OldPC :type Player%20Controller%20Object%20Reference) (NewPC :type Player%20Controller%20Object%20Reference))
  (Variables|Default|SetNew%20PC NewPC)
  (Development|PrintString "Swapped player controller")
  (Utilities|Casting|CastToBP_ThirdPersonPlayerController OldPC)
  (bind _asbp_game_instance_eos (Utilities|Casting|CastToBP_GameInstanceEOS (Game|GetGameInstance)))
  (if (Utilities|Enum|Equal(Enum) (Class|EOSGameInstance|GetSessionState _asbp_game_instance_eos) "PlayAgain")
    (Development|PrintString "PlayAgain in GameInstance")
    (Development|PrintString (Class|EOSGameInstance|GetSelectedGameMode _asbp_game_instance_eos))
    (switch string (Class|EOSGameInstance|GetSelectedGameMode _asbp_game_instance_eos)
      (:0
        (Development|PrintString "1v1")
        (bind _output_get (Variables|Default|SetMatchPlayersJoined (+ 1 (Variables|Default|GetMatchPlayersJoined))))
        (Development|PrintString (Utilities|String|Append "Players joined:" (Utilities|String|ToString(Integer) _output_get)))
        (if (== _output_get 2)
          (Development|PrintString "ROS Travel to Match Level" :!label _label)
          (Utilities|FlowControl|Delay 1.0)
          (CallFunction|ROSTraveltoMatchLevel)))
      (:1
        (Development|PrintString "2v2")
        (bind _output_get_2 (Variables|Default|SetMatchPlayersJoined (+ 1 (Variables|Default|GetMatchPlayersJoined))))
        (Development|PrintString (Utilities|String|Append "Players joined:" (Utilities|String|ToString(Integer) _output_get_2)))
        (if (== _output_get_2 4)
          (goto _label)))
      (:2
        (Development|PrintString "3v3")
        (bind _output_get_3 (Variables|Default|SetMatchPlayersJoined (+ 1 (Variables|Default|GetMatchPlayersJoined))))
        (Development|PrintString (Utilities|String|Append "Players joined:" (Utilities|String|ToString(Integer) _output_get_3)))
        (if (== _output_get_3 6)
          (goto _label))))
    (else
      (Development|PrintString "PlayAgain NOT in GameInstance")
      (if (Ability|HasAuthority (Variables|Default|GetNew%20PC))
        (if (Utilities|Enum|Equal(Enum) (Class|EOSGameInstance|GetSessionState _asbp_game_instance_eos) "ReturningToLobbyFromMatch")
          (Class|EOSGameInstance|ResetLobbySettings _asbp_game_instance_eos)
          (CallFunction|HandlePlayerEnteringLobby (Variables|Default|GetNew%20PC) :!label _label_2)
          (bind _asbp_lobby_game_state (Utilities|Casting|CastToBP_LobbyGameState (Game|GetGameState)))
          (Variables|/Game/Core/GameModes/Lobby/BP_LobbyGameState.BP_LobbyGameState_C|SetConnectedLobbyPlayers _asbp_lobby_game_state (Utilities|Array|Length (Variables|Default|GetPlayerControllers)))
          (Utilities|IfPlayerSlotsSet
            (:true
              (CallFunction|UpdatePlayerSlots)
              (bind _asbp_game_instance_eos_2 (Utilities|Casting|CastToBP_GameInstanceEOS (Game|GetGameInstance)))
              (if (not (or (Utilities|Enum|Equal(Enum) (Class|EOSGameInstance|GetSessionState _asbp_game_instance_eos_2) "JoiningMatch") (Utilities|Enum|Equal(Enum) (Class|EOSGameInstance|GetSessionState _asbp_game_instance_eos_2) "SearchingForMatch")))
                (bind _asbp_lobby_controller (Utilities|Casting|CastToBP_LobbyController (Game|GetPlayerController 0)))
                (Utilities|IsValid (Variables|/Game/Core/GameModes/Lobby/BP_LobbyController.BP_LobbyController_C|GetLobby%20UI _asbp_lobby_controller)
                  (:Is%20Valid
                    (Default|UpdateAvailableGameModes (Variables|/Game/Core/GameModes/Lobby/BP_LobbyController.BP_LobbyController_C|GetLobby%20UI _asbp_lobby_controller)))
                  (:Is%20Not%20Valid
                    (Development|PrintString "LobbyUI invalid"))))))
          (else
            (Development|PrintString "Was not in a match")))
        (else
          (goto _label_2))))))

(event EventPostLogin
  (params (NewPlayer :type Player%20Controller%20Object%20Reference))
  (Development|PrintString "OnPostLogin")
  (CallFunction|HandlePlayerEnteringLobby NewPlayer)
  (bind _asbp_lobby_game_state (Utilities|Casting|CastToBP_LobbyGameState (Game|GetGameState)))
  (Variables|/Game/Core/GameModes/Lobby/BP_LobbyGameState.BP_LobbyGameState_C|SetConnectedLobbyPlayers _asbp_lobby_game_state (Utilities|Array|Length (Variables|Default|GetPlayerControllers)))
  (Utilities|IfPlayerSlotsSet
    (:true
      (CallFunction|UpdatePlayerSlots)
      (bind _asbp_game_instance_eos (Utilities|Casting|CastToBP_GameInstanceEOS (Game|GetGameInstance)))
      (if (not (or (Utilities|Enum|Equal(Enum) (Class|EOSGameInstance|GetSessionState _asbp_game_instance_eos) "JoiningMatch") (Utilities|Enum|Equal(Enum) (Class|EOSGameInstance|GetSessionState _asbp_game_instance_eos) "SearchingForMatch")))
        (bind _asbp_lobby_controller (Utilities|Casting|CastToBP_LobbyController (Game|GetPlayerController 0)))
        (Utilities|IsValid (Variables|/Game/Core/GameModes/Lobby/BP_LobbyController.BP_LobbyController_C|GetLobby%20UI _asbp_lobby_controller)
          (:Is%20Valid
            (Default|UpdateAvailableGameModes (Variables|/Game/Core/GameModes/Lobby/BP_LobbyController.BP_LobbyController_C|GetLobby%20UI _asbp_lobby_controller)))
          (:Is%20Not%20Valid
            (Development|PrintString "LobbyUI invalid")))))))

(event EventOnLogout
  (params (ExitingController :type Controller%20Object%20Reference))
  (Development|PrintString "OnPostLogout")
  (CallFunction|HandlePlayerExitingGame ExitingController)
  (bind _asbp_lobby_game_state (Utilities|Casting|CastToBP_LobbyGameState (Game|GetGameState)))
  (Variables|/Game/Core/GameModes/Lobby/BP_LobbyGameState.BP_LobbyGameState_C|SetConnectedLobbyPlayers _asbp_lobby_game_state (Utilities|Array|Length (Variables|Default|GetPlayerControllers)))
  (Utilities|IfPlayerSlotsSet
    (:true
      (CallFunction|UpdatePlayerSlots)
      (bind _asbp_game_instance_eos (Utilities|Casting|CastToBP_GameInstanceEOS (Game|GetGameInstance)))
      (if (not (or (Utilities|Enum|Equal(Enum) (Class|EOSGameInstance|GetSessionState _asbp_game_instance_eos) "JoiningMatch") (Utilities|Enum|Equal(Enum) (Class|EOSGameInstance|GetSessionState _asbp_game_instance_eos) "SearchingForMatch")))
        (bind _asbp_lobby_controller (Utilities|Casting|CastToBP_LobbyController (Game|GetPlayerController 0)))
        (Utilities|IsValid (Variables|/Game/Core/GameModes/Lobby/BP_LobbyController.BP_LobbyController_C|GetLobby%20UI _asbp_lobby_controller)
          (:Is%20Valid
            (Default|UpdateAvailableGameModes (Variables|/Game/Core/GameModes/Lobby/BP_LobbyController.BP_LobbyController_C|GetLobby%20UI _asbp_lobby_controller)))
          (:Is%20Not%20Valid
            (Development|PrintString "LobbyUI invalid")))))))

(fn ConstructionScript)

(fn SetPlayerSlots
  (bind _outactors (Actor|GetAllActorsOfClass "/Game/Core/GameModes/Lobby/Assets/BP_PlayerSlot.BP_PlayerSlot_C"))
  (for _index (range 0 (Utilities|Array|LastIndex _outactors))
    (bind _outactors_2 (Actor|GetAllActorsOfClasswithTag "/Game/Core/GameModes/Lobby/Assets/BP_PlayerSlot.BP_PlayerSlot_C" (Utilities|String|StringToName (Utilities|String|ToString(Integer) _index))))
    (Utilities|Array|Add (Variables|Default|GetPlayer%20Slots) (Utilities|Array|Get(acopy) _outactors_2)))
  (Variables|Default|SetSetSlotsDone true))

(fn UpdatePlayerSlots
  ;[0.15 0.15 0.15 0.5] Check if player controller is already added
  (for _array_element (Variables|Default|GetPlayerControllers)
    (LocalVariables|SetPlayerControllerAlreadyAdded false)
    (bind _array_element_2 (Utilities|Array|ForEachLoopwithBreak (Variables|Default|GetPlayer%20Slots) :!label _label)
      (:LoopBody
        (if (== (Variables|/Game/Core/GameModes/Lobby/Assets/BP_PlayerSlot.BP_PlayerSlot_C|GetPlayerController _array_element_2) _array_element)
          (LocalVariables|SetPlayerControllerAlreadyAdded true)
          (goto _label Break)))
      (:Completed
        ;[0.15 0.15 0.15 0.5] Add player controller to player slot
        (if (not (LocalVariables|GetPlayerControllerAlreadyAdded))
          (bind _array_element_3 (Utilities|Array|ForEachLoopwithBreak (Variables|Default|GetPlayer%20Slots) :!label _label_2)
            (:LoopBody
              (Variables|/Game/Core/GameModes/Lobby/Assets/BP_PlayerSlot.BP_PlayerSlot_C|GetPlayerController _array_element_3
                (:then)
                (:else
                  (Default|AddPlayer _array_element_3 _array_element)
                  (goto _label_2 Break)))))))))
  (for _array_element_4 (Variables|Default|GetPlayer%20Slots)
    (if (not (Utilities|Array|ContainsItem (Variables|Default|GetPlayerControllers) (Variables|/Game/Core/GameModes/Lobby/Assets/BP_PlayerSlot.BP_PlayerSlot_C|GetPlayerController _array_element_4)))
      (Default|RemovePlayer _array_element_4))))

(fn CheckAllPlayersReady
  (LocalVariables|SetAllPlayersReady true)
  (for _array_element (Variables|Default|GetPlayerControllers)
    (bind _asbp_player_state (Utilities|Casting|CastToBP_PlayerState (Variables|/Script/Engine.Controller|GetPlayerState _array_element))
      (:then
        (if (Variables|/Game/Core/GameModes/Game/BP_PlayerState.BP_PlayerState_C|GetbLobby_IsPlayerReady _asbp_player_state)
          (Development|PrintString "Lobby player is ready")
          (else
            (LocalVariables|SetAllPlayersReady false)
            (Development|PrintString "player is not ready"))))
      (:CastFailed
        (Development|PrintString "player state cast failed"))))
  (bind _asbp_lobby_controller (Utilities|Casting|CastToBP_LobbyController (Game|GetPlayerController 0)))
  (Default|EnableFindMatch (Variables|/Game/Core/GameModes/Lobby/BP_LobbyController.BP_LobbyController_C|GetLobby%20UI _asbp_lobby_controller) (LocalVariables|GetAllPlayersReady))
  (Development|PrintString (Utilities|String|Append "All player are ready: " (Utilities|String|ToString(Boolean) (LocalVariables|GetAllPlayersReady)))))

(fn ReAddGameModeonLogout
  (Utilities|FlowControl|Sequence
    (:then_0
      (bind _array_element (Utilities|Array|ForEachLoopwithBreak (Variables|Default|GetAllGameModes) :!label _label)
        (:LoopBody
          (if (not (Utilities|Array|ContainsItem (Variables|Default|GetAvailableGameModes) (Utilities|Enum|ByteToEnumE_GameModes _array_element)))
            (Utilities|Array|Add (Variables|Default|GetAvailableGameModes) (Utilities|Enum|ByteToEnumE_GameModes _array_element))
            (Development|PrintString (Utilities|String|Append "Adding game mode to available game modes: " (Utilities|String|EnumtoString (Utilities|Enum|ByteToEnumE_GameModes _array_element))))
            (goto _label Break)))))
    (:then_1
      (return))))

(fn PlayingSolo
  (return (== (Utilities|Array|Length (Variables|Default|GetAllGameModes)) (Utilities|Array|Length (Variables|Default|GetAvailableGameModes)))))

(fn HandleJoiningOpponents
  (bind _result (Math|Integer|IncrementInt (Variables|Default|GetMatchOpponentsJoined))
    (:%20%20
      (Variables|Default|SetMatchOpponentsJoined _result)
      (switch Utilities|FlowControl|Switch|SwitchonE_GameModes (Variables|Default|GetSelectedGameMode)
        (:NewEnumerator0
          (if (== (Variables|Default|GetMatchOpponentsJoined) 1)
            (Development|PrintString "All oponents have joined" :!label _label)
            (CallFunction|ROSTraveltoMatchLevel)))
        (:NewEnumerator1
          (if (== (Variables|Default|GetMatchOpponentsJoined) 2)
            (goto _label)))
        (:NewEnumerator2
          (if (== (Variables|Default|GetMatchOpponentsJoined) 3)
            (goto _label)))))))

(fn CheckforHosttoJoinMatch
  (bind _result (Math|Integer|IncrementInt (Variables|Default|GetLobbyMembersJoinedMatch))
    (:%20%20
      (Variables|Default|SetLobbyMembersJoinedMatch _result)
      (switch Utilities|FlowControl|Switch|SwitchonE_GameModes (Variables|Default|GetSelectedGameMode)
        (:NewEnumerator1
          (if (== (Variables|Default|GetLobbyMembersJoinedMatch) 1)
            (Development|PrintString "2v2 match")
            (Development|PrintString "All members have joined the match" :!label _label)
            (bind _asbp_game_instance_eos (Utilities|Casting|CastToBP_GameInstanceEOS (Game|GetGameInstance)))
            (Default|JoinMatch _asbp_game_instance_eos)))
        (:NewEnumerator2
          (if (== (Variables|Default|GetLobbyMembersJoinedMatch) 2)
            (Development|PrintString "3v3 match")
            (goto _label)))))))

(fn HandlePlayerEnteringLobby
  (params (New%20PC :type Player%20Controller%20Object%20Reference))
  (bind _playercontrollers (Variables|Default|GetPlayerControllers))
  (bind _availablegamemodes (Variables|Default|GetAvailableGameModes))
  (bind _playercontrollers_2 (Variables|Default|GetPlayerControllers))
  (bind _returnvalue (Utilities|Array|Length _playercontrollers_2))
  (Development|PrintString "HandlePlayerEnteringLobby called")
  (bind _asbp_game_instance_eos (Utilities|Casting|CastToBP_GameInstanceEOS (Game|GetGameInstance)))
  (if (Utilities|Enum|Equal(Enum) (Class|EOSGameInstance|GetSessionState _asbp_game_instance_eos) "SearchingForMatch")
    (Class|EOSGameInstance|SetSessionState _asbp_game_instance_eos "JoiningMatch")
    (bind _asbp_player_state (Utilities|Casting|CastToBP_PlayerState (Game|GetPlayerState 0)))
    (Default|ClientsShowLoadingScreen _asbp_player_state)
    (CallFunction|HandleJoiningOpponents :!label _label)
    (elif (Utilities|Enum|Equal(Enum) (Class|EOSGameInstance|GetSessionState _asbp_game_instance_eos) "JoiningMatch")
      (goto _label)
      (else
        (bind _asbp_lobby_controller (Utilities|Casting|CastToBP_LobbyController New%20PC))
        (Default|ClientSetTeamID _asbp_lobby_controller (Class|AdvancedSessionsLibrary|UniqueNetIdtoString (Class|AdvancedSessionsLibrary|GetUniqueNetID (Game|GetPlayerController 0))))
        (Utilities|FlowControl|Sequence
          (:then_0
            (Utilities|Array|Add _playercontrollers New%20PC)
            (if (> (Utilities|Array|Length _playercontrollers) 1)
              (Utilities|Array|RemoveIndex _availablegamemodes (Utilities|Array|LastIndex _availablegamemodes))))
          (:then_1
            (bind _asbp_game_instance_eos_2 (Utilities|Casting|CastToBP_GameInstanceEOS (Game|GetGameInstance)))
            (if (Utilities|Enum|Equal(Enum) (Class|EOSGameInstance|GetSessionState _asbp_game_instance_eos_2) "Lobby")
              (Class|EOSGameInstance|SetCurrentTeamSize _asbp_game_instance_eos_2 _returnvalue)
              (Development|PrintString (Utilities|String|Append "Team size set to: " (Utilities|String|ToString(Integer) _returnvalue)))
              (Default|ClientStopLoadingScreen _asbp_lobby_controller)
              (Development|PrintString "Player joined lobby")))
          (:then_2
            (bind _asbp_game_instance_eos_3 (Utilities|Casting|CastToBP_GameInstanceEOS (Game|GetGameInstance)))
            (bind _output_get (Variables|Default|SetPlayersInLobby (+ (Variables|Default|GetPlayersInLobby) 1)))
            (if (and (== _output_get (Class|EOSGameInstance|GetCurrentTeamSize _asbp_game_instance_eos_3)) (Utilities|Enum|Equal(Enum) (Class|EOSGameInstance|GetSessionState _asbp_game_instance_eos_3) "ReturningToLobbyFromMatch"))
              (Utilities|Time|ClearandInvalidateTimerbyHandle (Variables|Default|GetReturnToLobbyMemberJoinFail))
              (for _array_element (Variables|Default|GetPlayerControllers)
                (bind _asbp_lobby_controller_2 (Utilities|Casting|CastToBP_LobbyController _array_element))
                (Default|ClientStopLoadingScreen _asbp_lobby_controller_2))
              (Class|EOSGameInstance|SetSessionState _asbp_game_instance_eos_3 "Lobby")
              (Development|PrintString "All players joined after returning from match")))
          (:then_3
            (return)))))))

(fn HandlePlayerExitingGame
  (params (Exiting%20controller :type Controller%20Object%20Reference))
  (bind _playercontrollers (Variables|Default|GetPlayerControllers))
  (bind _returnvalue (Utilities|Array|Length _playercontrollers))
  (bind _asbp_game_instance_eos (Utilities|Casting|CastToBP_GameInstanceEOS (Game|GetGameInstance)))
  (if (Utilities|Enum|Equal(Enum) (Class|EOSGameInstance|GetSessionState _asbp_game_instance_eos) "JoiningMatch")
    (CallFunction|CheckforHosttoJoinMatch))
  (bind _asplayer_controller (Utilities|Casting|CastToPlayerController Exiting%20controller))
  (if (Utilities|Array|ContainsItem (Variables|Default|GetPlayerControllers) _asplayer_controller)
    (Utilities|Array|RemoveItem (Variables|Default|GetPlayerControllers) _asplayer_controller)
    (Utilities|FlowControl|Sequence
      (:then_0
        (CallFunction|ReAddGameModeonLogout))
      (:then_1
        (if (Utilities|Enum|Equal(Enum) (Class|EOSGameInstance|GetSessionState _asbp_game_instance_eos) "Lobby")
          (bind _asbp_game_instance_eos_2 (Utilities|Casting|CastToBP_GameInstanceEOS (Game|GetGameInstance)))
          (Class|EOSGameInstance|SetCurrentTeamSize _asbp_game_instance_eos_2 _returnvalue)
          (Development|PrintString (Utilities|String|Append "Team size set to: " (Utilities|String|ToString(Integer) _returnvalue)))))
      (:then_2
        (bind _asbp_player_state (Utilities|Casting|CastToBP_PlayerState (Game|GetPlayerState 0)))
        (Default|ClientsSetAllPlayersNotReady _asbp_player_state)))))