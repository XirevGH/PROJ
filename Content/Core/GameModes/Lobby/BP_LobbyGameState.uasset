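; Lobby game state that pushes replicated lobby info to clients as it changes.
; When the connected player count replicates, it finds the local lobby controller's UI and shows the leave-lobby option only if more than one player is present.
; When the game mode text replicates, non-authority instances broadcast an update event with the new text.
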(fn ConstructionScript)

(fn OnRepConnectedLobbyPlayers
  (bind _returnvalue (Game|GetPlayerController 0))
  (Utilities|IsValid _returnvalue
    (:Is%20Valid
      (bind _asbp_lobby_controller (Utilities|Casting|CastToBP_LobbyController _returnvalue))
      (Utilities|IsValid (Variables|/Game/Core/GameModes/Lobby/BP_LobbyController.BP_LobbyController_C|GetLobby%20UI _asbp_lobby_controller)
        (:Is%20Valid
          (Default|SetLeaveLobbyVisible (Variables|/Game/Core/GameModes/Lobby/BP_LobbyController.BP_LobbyController_C|GetLobby%20UI _asbp_lobby_controller) (> (Variables|Default|GetConnectedLobbyPlayers) 1)))))))

(fn OnRepGameModeText
  (Networking|SwitchHasAuthority
    (:Remote
      (Default|CallOnUpdateGameModeText (Variables|Default|GetGameModeText)))))