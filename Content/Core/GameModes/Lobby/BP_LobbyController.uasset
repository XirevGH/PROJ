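; Lobby player controller that shows the lobby UI and relays player choices.
; On BeginPlay the local controller opens the UI with mouse input and sends the class saved in the EOS game instance to the server.
; Server events write ready state, selected class and nameplate name to the PlayerState, with ready changes triggering the lobby GameMode's all-ready check.
; A separate event stores the team ID in the game instance.
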(event Custom|Server_SetPlayerReady
  (params (bIsReady :type Boolean))
  (bind _asbp_player_state (Utilities|Casting|CastToBP_PlayerState (Variables|GetPlayerState)))
  (Variables|/Game/Core/GameModes/Game/BP_PlayerState.BP_PlayerState_C|SetbLobby_IsPlayerReady _asbp_player_state bIsReady)
  (bind _asbp_lobby_game_mode (Utilities|Casting|CastToBP_LobbyGameMode (Game|GetGameMode)))
  (Default|CheckAllPlayersReady _asbp_lobby_game_mode))

(event Custom|SetTeamIDOnGameInstance
  (params (TeamID :type String))
  (bind _asbp_game_instance_eos (Utilities|Casting|CastToBP_GameInstanceEOS (Game|GetGameInstance)))
  (Variables|/Game/Core/BP_GameInstanceEOS.BP_GameInstanceEOS_C|SetTeamID _asbp_game_instance_eos TeamID))

(event Custom|Server_SwitchCharacterClass
  (params (CharacterClass :type E_CharacterClass%20Enum :default "NewEnumerator0"))
  (bind _asbp_player_state (Utilities|Casting|CastToBP_PlayerState (Variables|GetPlayerState)))
  (Variables|/Game/Core/GameModes/Game/BP_PlayerState.BP_PlayerState_C|SetSelectedClass _asbp_player_state CharacterClass))

(event Custom|Server_UpdatePlayerInfoName
  (bind _asbp_player_state (Utilities|Casting|CastToBP_PlayerState (Variables|GetPlayerState)))
  (Variables|/Game/Core/GameModes/Game/BP_PlayerState.BP_PlayerState_C|SetLobby_PlayerNameplateName _asbp_player_state (PlayerState|GetPlayerName _asbp_player_state)))

(event EventBeginPlay
  (if (Pawn|IsLocalPlayerController)
    (bind _returnvalue (UserInterface|CreateWidget "/Game/UI/Lobby/WBP_LobbyUI.WBP_LobbyUI_C"))
    (bind _output_get (Variables|Default|SetLobby%20UI _returnvalue))
    (UserInterface|Viewport|AddtoViewport _output_get 0)
    (Variables|Default|SetbShowMouseCursor true)
    (Input|SetInputModeGameandUI self (Variables|Default|GetLobby%20UI) "DoNotLock" true false)
    (bind _asbp_game_instance_eos (Utilities|Casting|CastToBP_GameInstanceEOS (Game|GetGameInstance)))
    (CallFunction|ServerSwitchCharacterClass (Variables|/Game/Core/BP_GameInstanceEOS.BP_GameInstanceEOS_C|GetCharacterClass _asbp_game_instance_eos))))

(fn ConstructionScript)