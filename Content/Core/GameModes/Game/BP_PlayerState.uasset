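; Player state shared by lobby and match that replicates team, class, ready, name and death state for each player.
; RepNotifies push changes to the lobby mannequin and info widget, character nameplate, and game state for player registration and deaths.
; Client events drive matchmaking UI and session joins through the EOS game instance.
; Team setup takes the game instance's TeamID for locally controlled pawns, then notifies the game mode of the join.
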(event Custom|ROS_LobbyMemberJoiningMatch
  (bind _asbp_lobby_game_mode (Utilities|Casting|CastToBP_LobbyGameMode (Game|GetGameMode)))
  (Default|ROSonLobbyMemberJoiningMatch _asbp_lobby_game_mode))

(event Custom|Client_JoinFoundMatch
  (params (SessionName :type String))
  (Networking|SwitchHasAuthority
    (:Remote
      (bind _asbp_game_instance_eos (Utilities|Casting|CastToBP_GameInstanceEOS (Game|GetGameInstance)))
      (Default|JoinMatch _asbp_game_instance_eos SessionName))))

(event Custom|Client_SearchingForMatch
  (bind _asbp_lobby_controller (Utilities|Casting|CastToBP_LobbyController (Game|GetPlayerController 0)))
  (Default|HandleIsSearchingforMatch (Variables|/Game/Core/GameModes/Lobby/BP_LobbyController.BP_LobbyController_C|GetLobby%20UI _asbp_lobby_controller)))

(event Custom|SetTeamID_Event
  (bind _asbp_game_instance_eos (Utilities|Casting|CastToBP_GameInstanceEOS (Game|GetGameInstance)))
  (Development|PrintString (Utilities|String|Append "Inside player state of " (PlayerState|GetPlayerName) ", the game instance reports TeamID of: " (Variables|/Game/Core/BP_GameInstanceEOS.BP_GameInstanceEOS_C|GetTeamID _asbp_game_instance_eos)))
  (if (Pawn|IsLocallyControlled (PlayerState|GetPawn))
    (CallFunction|ROSSetTeamID (Variables|/Game/Core/BP_GameInstanceEOS.BP_GameInstanceEOS_C|GetTeamID _asbp_game_instance_eos))
    (else
      (Development|PrintString "This player state is not locally controlled")))
  (bind _asbp_third_person_player_controller (Utilities|Casting|CastToBP_ThirdPersonPlayerController (Game|GetPlayerController)))
  (bind _asbp_base_game_mode (Utilities|Casting|CastToBP_BaseGameMode (Game|GetGameMode)))
  (Default|PlayerHasFullyJoined _asbp_base_game_mode _asbp_third_person_player_controller))

(event Custom|ROS_SetTeamID
  (params (TeamID :type String))
  (Development|PrintString (Utilities|String|Append "Inside PlayerState SetTeamID setting team ID to:  " TeamID))
  (Class|BasePlayerState|SetTeamID TeamID))

(event Custom|Client_CancelSearchingForMatch
  (bind _asbp_lobby_controller (Utilities|Casting|CastToBP_LobbyController (Game|GetPlayerController 0)))
  (Default|HandleCancelMatchSearch (Variables|/Game/Core/GameModes/Lobby/BP_LobbyController.BP_LobbyController_C|GetLobby%20UI _asbp_lobby_controller)))

(event EventBeginPlay
  (Development|PrintString "PlayerState begin play")
  (bind _asbp_third_person_player_controller (Utilities|Casting|CastToBP_ThirdPersonPlayerController (Game|GetPlayerController 0))
    (:then
      (Default|PlayerStateIsHere _asbp_third_person_player_controller self))
    (:CastFailed
      (Development|PrintString "TPPC cast failed"))))

(event EventOnRepTeamID
  (Development|PrintString "OnRep_TeamID fired")
  (bind _asbp_game_state (Utilities|Casting|CastToBP_GameState (Game|GetGameState))
    (:then
      (Default|RegisterPlayertoMap _asbp_game_state self))
    (:CastFailed
      (Development|PrintString "Failed GameState cast"))))

(fn ConstructionScript)

(fn LobbyUpdateIsReady
  (bind _aswbp_player_info (Utilities|Casting|CastToWBP_PlayerInfo (UserInterface|GetUserWidgetObject (Variables|/Game/Core/GameModes/Lobby/Assets/BP_LobbyMannequin.BP_LobbyMannequin_C|GetWidget_Lobby_PlayerInfo (Variables|Default|GetLobby_Mannequin)))))
  (Default|UpdatePlayerReady _aswbp_player_info (Variables|Default|GetbLobby_IsPlayerReady)))

(fn GameUpdatePlayerNameplate
  (Development|PrintString "UpdatePlayerNameplate run")
  (bind _asbp_third_person_character (Utilities|Casting|CastToBP_ThirdPersonCharacter (Pawn|GetControlledPawn (Variables|Default|GetPlayerController)))
    (:then
      (Development|PrintString (Utilities|GetDisplayName _asbp_third_person_character))
      (bind _aswbp_nameplate (Utilities|Casting|CastToWBP_Nameplate (UserInterface|GetUserWidgetObject (Variables|/Game/Characters/Base/_Core/BP_ThirdPersonCharacter.BP_ThirdPersonCharacter_C|GetNameplateWidget _asbp_third_person_character))))
      (Default|SetPlayerNameText (Variables|/Game/UI/Game/InGameWIdgets/WBP_Nameplate.WBP_Nameplate_C|GetWBP_OverheadName _aswbp_nameplate) (Variables|Default|GetGame_PlayerNameplateName)))
    (:CastFailed
      (Development|PrintString "Cast to TPChar failed"))))

(fn LobbyUpdatePlayerInfoName
  (bind _aswbp_player_info (Utilities|Casting|CastToWBP_PlayerInfo (UserInterface|GetWidget (Variables|/Game/Core/GameModes/Lobby/Assets/BP_LobbyMannequin.BP_LobbyMannequin_C|GetWidget_Lobby_PlayerInfo (Variables|Default|GetLobby_Mannequin)))))
  (Default|SetPlayerNameText _aswbp_player_info (Variables|Default|GetLobby_PlayerNameplateName)))

(fn OnRepBLobbyIsPlayerReady
  (CallFunction|LobbyUpdateIsReady))

(fn OnRepSelectedClass
  (Default|ServerUpdateCharacterDisplay (Variables|Default|GetLobby_Mannequin) (Variables|Default|GetSelectedClass)))

(fn OnRepLobbyMannequin
  (CallFunction|LobbyUpdateIsReady)
  (CallFunction|LobbyUpdatePlayerInfoName)
  (bind _asbp_lobby_controller (Utilities|Casting|CastToBP_LobbyController (Game|GetPlayerController)))
  (Default|ServerUpdatePlayerInfoName _asbp_lobby_controller)
  (Default|ServerSetPlayerReady _asbp_lobby_controller (Variables|Default|GetbLobby_IsPlayerReady)))

(fn OnRepGamePlayerNameplateName
  (bind _returnvalue (PlayerState|GetPawn))
  (Utilities|IsValid _returnvalue
    (:Is%20Valid
      (bind _asbp_third_person_character (Utilities|Casting|CastToBP_ThirdPersonCharacter _returnvalue)
        (:then
          (Default|SetNameServer _asbp_third_person_character (Variables|Default|GetGame_PlayerNameplateName)))
        (:CastFailed
          (Development|PrintString "Cast to TPChar failed"))))
    (:Is%20Not%20Valid
      (Development|PrintString "pawn not valid"))))

(fn OnRepLobbyPlayerNameplateName
  (CallFunction|LobbyUpdatePlayerInfoName))

(fn OnRepPlayerController
  (Development|PrintString "OnRep_PlayerController run")
  (CallFunction|GameUpdatePlayerNameplate))

(fn OnRepBIsDead
  (bind _asbp_game_state (Utilities|Casting|CastToBP_GameState (Game|GetGameState)))
  (Default|OnPlayerDied _asbp_game_state))