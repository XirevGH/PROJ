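; Base game mode for a two-team online match that assigns joining players to teams, moves them to team starts and tracks leavers.
; One-second timers run preparation and match countdowns through the game state, flagging a draw on timeout and stopping on team death.
; Restart and empty-team handling server-travel to the lobby.
; Return-to-lobby picks a leader for the non-host team and has its members migrate to a new EOS session.
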(event Custom|PreparationCountdown
  (bind _output_get (Variables|/Game/Core/GameModes/Game/BP_GameState.BP_GameState_C|SetPreparationTimeRemaining (Variables|Default|GetGameStateRef) (- (Variables|/Game/Core/GameModes/Game/BP_GameState.BP_GameState_C|GetPreparationTimeRemaining (Variables|Default|GetGameStateRef)) 1)))
  (if (<= _output_get 0)
    (Utilities|Time|ClearandInvalidateTimerbyHandle (Variables|Default|GetPreparationTimerHandle))
    (Utilities|FlowControl|Sequence
      (:then_0
        (Default|CallOnPreparationComplete (Variables|Default|GetGameStateRef))
        (EventDispatchers|AssignOnTeamDeath (Variables|Default|GetGameStateRef) (delegate Custom|OnTeamDeath)))
      (:then_1
        (bind _returnvalue (Utilities|Time|SetTimerbyEvent (delegate Custom|MatchCountdown) 1.0 true))
        (Variables|Default|SetMatchTimerHandle _returnvalue)))))

(event Custom|MatchCountdown
  (bind _output_get (Variables|/Game/Core/GameModes/Game/BP_GameState.BP_GameState_C|SetMatchTimeRemaining (Variables|Default|GetGameStateRef) (- (Variables|/Game/Core/GameModes/Game/BP_GameState.BP_GameState_C|GetMatchTimeRemaining (Variables|Default|GetGameStateRef)) 1)))
  (if (<= _output_get 0)
    (Utilities|Time|ClearandInvalidateTimerbyHandle (Variables|Default|GetMatchTimerHandle))
    (Variables|/Game/Core/GameModes/Game/BP_GameState.BP_GameState_C|SetMatchDraw (Variables|Default|GetGameStateRef) true)))

(event Custom|Event_OnTeamEmpty
  (params (EmptyTeamID :type String))
  (Development|PrintString "Other team have left")
  (Development|PrintString "Returning to lobby")
  (if (Variables|Default|GetReturnToLobbyCalled)
    _
    (else
      (bind _asbp_game_instance_eos (Utilities|Casting|CastToBP_GameInstanceEOS (Game|GetGameInstance)))
      (Class|EOSGameInstance|SetSessionState _asbp_game_instance_eos "ReturningToLobbyFromMatch")
      (bind _asbp_player_state (Utilities|Casting|CastToBP_PlayerState (Game|GetPlayerState 0)))
      (Default|ClientsShowLoadingScreen _asbp_player_state)))
  (Class|AdvancedSessionsLibrary|ServerTravel "/Game/Levels/Lvl_Lobby" false false))

(event Custom|PlayerHasFullyJoined
  (params (Player%20controller :type BP%20Third%20Person%20Player%20Controller%20Object%20Reference))
  (Development|PrintString (Utilities|String|Append (Class|AdvancedSessionsLibrary|GetPlayerName Player%20controller) " has fully joined "))
  (bind _asbp_player_state (Utilities|Casting|CastToBP_PlayerState (Variables|/Script/Engine.Controller|GetPlayerState Player%20controller)))
  (CallFunction|AssignPlayerTeam (Variables|/Game/Core/GameModes/Game/BP_PlayerState.BP_PlayerState_C|GetTeamID _asbp_player_state) Player%20controller)
  (Default|ClientsStopLoadingScreen _asbp_player_state))

(event Custom|OnTeamDeath
  (Utilities|Time|ClearandInvalidateTimerbyHandle (Variables|Default|GetMatchTimerHandle)))

(event Custom|Event_RestartMatch
  (bind _playagaindelay (Variables|Default|GetPlayAgainDelay))
  (Development|PrintString "Event_RestartMatch")
  (bind _asbp_player_state (Utilities|Casting|CastToBP_PlayerState (Game|GetPlayerState 0)))
  (Default|ClientsPrepareforMatchConclusionAction _asbp_player_state false (Math|Float|Truncate _playagaindelay))
  (Utilities|FlowControl|Delay (+ _playagaindelay 0.5))
  (CallFunction|RestartMatch))

(event Custom|Event_ReturnToLobby
  (bind _returntolobbydelay (Variables|Default|GetReturnToLobbyDelay))
  (Development|PrintString "Event_ReturnToLobby")
  (bind _asbp_player_state (Utilities|Casting|CastToBP_PlayerState (Game|GetPlayerState 0)))
  (Default|ClientsPrepareforMatchConclusionAction _asbp_player_state true (Math|Float|Truncate _returntolobbydelay))
  (Utilities|FlowControl|Delay (+ _returntolobbydelay 0.5))
  (CallFunction|ReturntoLobby))

(event EventBeginPlay
  (Development|PrintString "BeginPlay")
  (Utilities|FlowControl|Sequence
    (:then_0
      (bind _asbp_game_state (Utilities|Casting|CastToBP_GameState (Game|GetGameState)))
      (bind _output_get (Variables|Default|SetGameStateRef _asbp_game_state))
      (Variables|/Game/Core/GameModes/Game/BP_GameState.BP_GameState_C|SetPreparationTimeRemaining _output_get (Variables|Default|GetPreparationTimer))
      (Variables|/Game/Core/GameModes/Game/BP_GameState.BP_GameState_C|SetMatchTimeRemaining _output_get (Variables|Default|GetMatchTimer))
      (bind _returnvalue (Utilities|Time|SetTimerbyEvent (delegate Custom|PreparationCountdown) 1.0 true))
      (Variables|Default|SetPreparationTimerHandle _returnvalue))
    (:then_1
      (EventDispatchers|BindEventtoOnTeamEmpty (delegate Custom|Event_OnTeamEmpty)))))

(event EventOnLogout
  (params (ExitingController :type Controller%20Object%20Reference))
  (bind _asbp_third_person_player_controller (Utilities|Casting|CastToBP_ThirdPersonPlayerController ExitingController))
  (bind _asbp_player_state (Utilities|Casting|CastToBP_PlayerState (Variables|/Script/Engine.Controller|GetPlayerState ExitingController)))
  (Development|PrintString (Utilities|String|Append "Player left from team: " (Variables|/Game/Core/GameModes/Game/BP_PlayerState.BP_PlayerState_C|GetTeamID _asbp_player_state)))
  (Class|BaseGameMode|RemovePlayerfromTeam (Variables|/Game/Core/GameModes/Game/BP_PlayerState.BP_PlayerState_C|GetTeamID _asbp_player_state) _asbp_third_person_player_controller))

(event EventOnSwapPlayerControllers
  (params (OldPC :type Player%20Controller%20Object%20Reference) (NewPC :type Player%20Controller%20Object%20Reference))
  (bind _asbp_third_person_player_controller (Utilities|Casting|CastToBP_ThirdPersonPlayerController NewPC))
  (Default|SetCharacterClass _asbp_third_person_player_controller))

(event EventOnPlayerArrived
  (params (C :type Controller%20Object%20Reference))
  (bind _asbp_game_instance_eos (Utilities|Casting|CastToBP_GameInstanceEOS (Game|GetGameInstance)))
  (if (Utilities|Enum|Equal(Enum) (Class|EOSGameInstance|GetSessionState _asbp_game_instance_eos) "Lobby")
    (Development|PrintString "Seamless travel from match to match")
    (bind _asbp_third_person_player_controller (Utilities|Casting|CastToBP_ThirdPersonPlayerController C)
      (:then
        (bind _asbp_player_state (Utilities|Casting|CastToBP_PlayerState (Variables|/Script/Engine.Controller|GetPlayerState C))
          (:then
            (Class|BaseGameMode|AddPlayertoTeam (Variables|/Game/Core/GameModes/Game/BP_PlayerState.BP_PlayerState_C|GetTeamID _asbp_player_state) _asbp_third_person_player_controller)
            (Default|ClientInitializePlayer _asbp_third_person_player_controller))
          (:CastFailed
            (Development|PrintString "Failed cast to player state"))))
      (:CastFailed
        (Development|PrintString "Failed cast to third person controller")))
    (else
      (Development|PrintString "Seamless travel from not in match"))))

(fn ConstructionScript)

(fn FindPlayerStartbyIndex
  (params (Index :type Integer))
  (bind _outactors (Actor|GetAllActorsOfClass "/Script/Engine.PlayerStart"))
  (return (Transformation|GetActorTransform (Utilities|Array|Get(acopy) _outactors Index))))

(fn SpawnPlayer
  (params (Player%20Controller :type Player%20Controller%20Object%20Reference) (CharacterClass :type E_CharacterClass%20Enum :default "NewEnumerator0"))
  (bind _returnvalue (Pawn|GetControlledPawn Player%20Controller))
  (bind _returnvalue_2 (Utilities|GetDataTableRow "/Game/Core/GameModes/Lobby/Assets/DT_CharacterLobbyData.DT_CharacterLobbyData" (Utilities|String|StringToName (Utilities|String|EnumtoString CharacterClass)))
    (:then
      (if (Utilities|IsValidClass (.characterclass _returnvalue_2))
        (Utilities|IsValid _returnvalue
          (:Is%20Valid
            (Actor|DestroyActor _returnvalue))
          (:Is%20Not%20Valid
            _))
        (bind _returnvalue_3 (Game|SpawnActorfromClass (.characterclass _returnvalue_2) (Math|Transform|MakeTransform "0, 0, 0") "AlwaysSpawn" "MultiplyWithRoot" 0 0))
        (Pawn|Possess Player%20Controller _returnvalue_3)
        (Development|PrintString "Team 1 player possessed")
        (Development|PrintString (Utilities|GetDisplayName (Pawn|GetControlledPawn Player%20Controller)))
        (else
          (Development|PrintString "Trying to spawn player with invalid class"))))))

(fn ReturntoLobby
  (bind _otherteamplayers (LocalVariables|GetOtherTeamPlayers))
  (bind _output (Utilities|Array|Get(acopy) _otherteamplayers))
  (Variables|Default|SetReturnToLobbyCalled true)
  (bind _asbp_game_instance_eos (Utilities|Casting|CastToBP_GameInstanceEOS (Game|GetGameInstance)))
  (Class|EOSGameInstance|SetSessionState _asbp_game_instance_eos "ReturningToLobbyFromMatch")
  (bind _asbp_player_state (Utilities|Casting|CastToBP_PlayerState (Game|GetPlayerState 0)))
  (Default|ClientsShowLoadingScreen _asbp_player_state)
  (Utilities|FlowControl|Sequence
    (:then_0
      (bind _array_element (Utilities|Array|ForEachLoopwithBreak (Variables|Default|GetTeamIDs) :!label _label)
        (:LoopBody
          (bind _returnvalue (Class|BaseGameMode|GetPlayersinTeam _array_element))
          (bind _asbp_third_person_player_controller (Utilities|Casting|CastToBP_ThirdPersonPlayerController (Game|GetPlayerController 0))
            (:then
              (if (Utilities|Array|ContainsItem _returnvalue _asbp_third_person_player_controller)
                (Development|PrintString (Utilities|String|Append "Skipped server team with ID: " _array_element))
                (else
                  (Development|PrintString (Utilities|String|Append "Other TeamID is " _array_element))
                  (for _array_element_2 _returnvalue
                    (bind _asbp_third_person_player_controller_2 (Utilities|Casting|CastToBP_ThirdPersonPlayerController _array_element_2)
                      (:then
                        (Utilities|Array|Add (LocalVariables|GetOtherTeamPlayers) _asbp_third_person_player_controller_2)
                        (Development|PrintString "Added controller to other team array")
                        (goto _label Break))
                      (:CastFailed
                        (Development|PrintString "Failed cast to third person player controller")))))))
            (:CastFailed
              (Development|PrintString "Failed cast to thirs person player controller"))))
        (:Completed
          (Development|PrintString (Utilities|String|Append "Players in other team: " (Utilities|String|ToString(Integer) (Utilities|Array|Length (LocalVariables|GetOtherTeamPlayers))))))))
    (:then_1
      (bind _array_element_3 (Utilities|Array|ForEachLoopwithBreak (LocalVariables|GetOtherTeamPlayers) :!label _label_2)
        (:LoopBody
          (if (Variables|/Game/Core/GameModes/Game/BP_ThirdPersonPlayerController.BP_ThirdPersonPlayerController_C|GetbIsTeamLeader _array_element_3)
            (Development|PrintString "Leader found")
            (LocalVariables|SetOtherTeamLeader _array_element_3)
            (Utilities|Array|RemoveItem (LocalVariables|GetOtherTeamPlayers) _array_element_3)
            (goto _label_2 Break)))))
    (:then_2
      (bind _otherteamleader (LocalVariables|GetOtherTeamLeader)
        (:then
          (bind _output_get (LocalVariables|SetSessionName (Utilities|String|Append (PlayerState|GetPlayerName (Variables|/Script/Engine.Controller|GetPlayerState _otherteamleader)) "_" (Guid|ToString(Guid) (Guid|NewGuid)))))
          (Development|PrintString (Utilities|String|Append "SessionName: " _output_get))
          (Default|ClientStartLeaderMigration _otherteamleader _output_get))
        (:else
          (Development|PrintString "Other leader is not valid")
          (Development|PrintString "Selecting new leader")
          (Utilities|IsValid _output
            (:Is%20Valid
              (bind _output_get_2 (LocalVariables|SetSessionName (Utilities|String|Append (PlayerState|GetPlayerName (Variables|/Script/Engine.Controller|GetPlayerState _output)) "_" (Guid|ToString(Guid) (Guid|NewGuid)))))
              (Development|PrintString (Utilities|String|Append "SessionName: " _output_get_2))
              (Default|ClientStartLeaderMigration _output _output_get_2)
              (Development|PrintString "Called StartLeaderMigration on the lerader")
              (Utilities|Array|RemoveItem (LocalVariables|GetOtherTeamPlayers) _output))
            (:Is%20Not%20Valid
              (Development|PrintString "Player with index 0 is not valid"))))))
    (:then_3
      (for _array_element_4 (LocalVariables|GetOtherTeamPlayers)
        (if (not (Variables|/Game/Core/GameModes/Game/BP_ThirdPersonPlayerController.BP_ThirdPersonPlayerController_C|GetbIsTeamLeader _array_element_4))
          (Default|ClientStartMemberMigration _array_element_4 (LocalVariables|GetSessionName))
          (Development|PrintString "Called StartMemberMigration on other team member"))))))

(fn AssignPlayerTeam
  (params (TeamID :type String) (Player%20controller :type BP%20Third%20Person%20Player%20Controller%20Object%20Reference))
  (bind _teamids (Variables|Default|GetTeamIDs))
  (Development|PrintString (Utilities|String|Append "AssignPlayerTeam: Team ID is:" TeamID))
  (Class|BaseGameMode|AddPlayertoTeam TeamID Player%20controller)
  (if (Utilities|Array|ContainsItem (Variables|Default|GetTeamIDs) TeamID)
    (Development|PrintString "The ID already existed in the Team IDs array")
    (else
      (Development|PrintString "The ID did not exist, it is being added now.")
      (Utilities|Array|Add (Variables|Default|GetTeamIDs) TeamID)))
  (bind _asbp_game_state (Utilities|Casting|CastToBP_GameState (Game|GetGameState)))
  (for _array_element _teamids
    (Development|PrintString (Utilities|String|Append "Team is in Team Ids array: " _array_element))
    (Utilities|FlowControl|Sequence
      (:then_0
        (if (Utilities|Array|IsValidIndex _teamids 1)
          (Variables|/Game/Core/GameModes/Game/BP_GameState.BP_GameState_C|SetTeamTwo _asbp_game_state (Utilities|Array|Get(acopy) _teamids 1))
          (else
            (Variables|/Game/Core/GameModes/Game/BP_GameState.BP_GameState_C|SetTeamOne _asbp_game_state (Utilities|Array|Get(acopy) _teamids)))))
      (:then_1
        (bind _asbp_third_person_character (Utilities|Casting|CastToBP_ThirdPersonCharacter (Pawn|GetControlledPawn Player%20controller)))
        (CallFunction|PlacePlayeratTeamSpawnLocation _asbp_third_person_character)))))

(fn PlacePlayeratTeamSpawnLocation
  (params (PlayerCharacter :type BP%20Third%20Person%20Character%20Object%20Reference))
  (bind _teamid (Default|GetTeamID PlayerCharacter))
  (if (Utilities|Enum|Equal(Enum) _teamid (Utilities|Array|Get(acopy) (Variables|Default|GetTeamIDs)))
    (Transformation|SetActorTransform PlayerCharacter (CallFunction|FindPlayerStartbyIndex))
    (else
      (Transformation|SetActorTransform PlayerCharacter (CallFunction|FindPlayerStartbyIndex 1)))))

(fn RestartMatch
  (Development|PrintString "RestartMatch")
  (bind _asbp_game_instance_eos (Utilities|Casting|CastToBP_GameInstanceEOS (Game|GetGameInstance)))
  (Class|EOSGameInstance|SetSessionState _asbp_game_instance_eos "PlayAgain")
  (bind _asbp_player_state (Utilities|Casting|CastToBP_PlayerState (Game|GetPlayerState 0)))
  (Default|ClientsShowLoadingScreen _asbp_player_state)
  (Game|GetCurrentLevelName true)
  (Class|AdvancedSessionsLibrary|ServerTravel (Utilities|String|Append "/Game/Levels/" "Lvl_Lobby" "?listen") false false))