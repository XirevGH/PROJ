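; Test game mode for a two-team match, with debug prints throughout.
; On controller swap from lobby, it registers team IDs in GameState, though the incoming ID is left blank and the new controller's TeamID is cleared.
; BeginPlay chains one-second preparation and match countdowns through GameState, flagging a draw on timeout.
; SpawnPlayer replaces the pawn with BP_LoremIpsum or BP_Singularist by team, at an indexed PlayerStart.
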(event Custom|PreparationCountdown
  (bind _output_get (Variables|/Game/Core/GameModes/Game/BP_GameState.BP_GameState_C|SetPreparationTimeRemaining (Variables|Default|GetGameStateRef) (- (Variables|/Game/Core/GameModes/Game/BP_GameState.BP_GameState_C|GetPreparationTimeRemaining (Variables|Default|GetGameStateRef)) 1)))
  (if (<= _output_get 0)
    (Utilities|Time|ClearandInvalidateTimerbyHandle (Variables|Default|GetPreparationTimerHandle))
    (Utilities|FlowControl|Sequence
      (:then_0
        (Default|CallOnPreparationComplete (Variables|Default|GetGameStateRef)))
      (:then_1
        (bind _returnvalue (Utilities|Time|SetTimerbyEvent (delegate Custom|MatchCountdown) 1.0 true))
        (Variables|Default|SetMatchTimerHandle _returnvalue)))))

(event Custom|MatchCountdown
  (bind _output_get (Variables|/Game/Core/GameModes/Game/BP_GameState.BP_GameState_C|SetMatchTimeRemaining (Variables|Default|GetGameStateRef) (- (Variables|/Game/Core/GameModes/Game/BP_GameState.BP_GameState_C|GetMatchTimeRemaining (Variables|Default|GetGameStateRef)) 1)))
  (if (<= _output_get 0)
    (Utilities|Time|ClearandInvalidateTimerbyHandle (Variables|Default|GetMatchTimerHandle))
    (Variables|/Game/Core/GameModes/Game/BP_GameState.BP_GameState_C|SetMatchDraw (Variables|Default|GetGameStateRef) true)))

(event EventBeginPlay
  (bind _asbp_game_state (Utilities|Casting|CastToBP_GameState (Game|GetGameState)))
  (bind _output_get (Variables|Default|SetGameStateRef _asbp_game_state))
  (Variables|/Game/Core/GameModes/Game/BP_GameState.BP_GameState_C|SetPreparationTimeRemaining _output_get (Variables|Default|GetPreparationTimer))
  (Variables|/Game/Core/GameModes/Game/BP_GameState.BP_GameState_C|SetMatchTimeRemaining _output_get (Variables|Default|GetMatchTimer))
  (bind _returnvalue (Utilities|Time|SetTimerbyEvent (delegate Custom|PreparationCountdown) 1.0 true))
  (Variables|Default|SetPreparationTimerHandle _returnvalue))

(event EventOnSwapPlayerControllers
  (params (OldPC :type Player%20Controller%20Object%20Reference) (NewPC :type Player%20Controller%20Object%20Reference))
  (bind _teamids (Variables|Default|GetTeamIDs))
  (Utilities|Casting|CastToBP_LobbyController OldPC)
  (Development|PrintString (Utilities|String|Append "LobbyController reports TeamID: " ""))
  (if (Utilities|Array|ContainsItem (Variables|Default|GetTeamIDs) "")
    (Development|PrintString "The ID already existed in the Team IDs array")
    (else
      (Development|PrintString "The ID did not exist, it is being added now.")
      (Utilities|Array|Add (Variables|Default|GetTeamIDs) "")))
  (bind _asbp_game_state (Utilities|Casting|CastToBP_GameState (Game|GetGameState))
    (:then
      (if (Utilities|Array|IsValidIndex _teamids 1)
        (Development|PrintString "index 1 in the array is valid, it must be Team Two")
        (bind _output_get (Variables|/Game/Core/GameModes/Game/BP_GameState.BP_GameState_C|SetTeamTwo _asbp_game_state (Utilities|Array|Get(acopy) _teamids 1)))
        (Development|PrintString (Utilities|String|Append "TeamTwoID: " _output_get))
        (else
          (Development|PrintString "index 1 in the array is not valid, Team Two has not been aded yet, it has to be Team One")
          (bind _output_get_2 (Variables|/Game/Core/GameModes/Game/BP_GameState.BP_GameState_C|SetTeamOne _asbp_game_state (Utilities|Array|Get(acopy) _teamids)))
          (Development|PrintString (Utilities|String|Append "TeamOneID: " _output_get_2))))
      (bind _asbp_third_person_player_controller (Utilities|Casting|CastToBP_ThirdPersonPlayerController NewPC))
      (Development|PrintString (Utilities|String|Append "ID before adding: " ""))
      (bind _output_get_3 (Variables|/Game/Core/GameModes/Game/BP_ThirdPersonPlayerController.BP_ThirdPersonPlayerController_C|SetTeamID _asbp_third_person_player_controller ""))
      (Development|PrintString (Utilities|String|Append "TeamID " _output_get_3 " is being set on the playercontroller")))
    (:CastFailed
      (Development|PrintString "Failed cast to gamestate"))))

(fn ConstructionScript)

(fn FindPlayerStartbyIndex
  (params (Index :type Integer))
  (bind _outactors (Actor|GetAllActorsOfClass "/Script/Engine.PlayerStart"))
  (return (Transformation|GetActorTransform (Utilities|Array|Get(acopy) _outactors Index))))

(fn SpawnPlayer
  (params (Player%20Controller :type Player%20Controller%20Object%20Reference))
  (bind _returnvalue (Pawn|GetControlledPawn Player%20Controller))
  (bind _asbp_third_person_player_controller (Utilities|Casting|CastToBP_ThirdPersonPlayerController Player%20Controller))
  (Utilities|IsValid _returnvalue
    (:Is%20Valid
      (Actor|DestroyActor _returnvalue))
    (:Is%20Not%20Valid
      _))
  (if (Utilities|Enum|Equal(Enum) (Variables|/Game/Core/GameModes/Game/BP_ThirdPersonPlayerController.BP_ThirdPersonPlayerController_C|GetTeamID _asbp_third_person_player_controller) (Utilities|Array|Get(acopy) (Variables|Default|GetTeamIDs)))
    (Development|PrintString "team 1")
    (bind _returnvalue_2 (Game|SpawnActorfromClass "/Game/Characters/LoremIpsum/_Core/BP_LoremIpsum.BP_LoremIpsum_C" (CallFunction|FindPlayerStartbyIndex) "AlwaysSpawn" "MultiplyWithRoot" 0 0))
    (Pawn|Possess Player%20Controller _returnvalue_2)
    (Development|PrintString "Team 1 player possessed")
    (Development|PrintString (Utilities|GetDisplayName (Pawn|GetControlledPawn Player%20Controller)))
    (else
      (Development|PrintString "team 2")
      (bind _returnvalue_3 (Game|SpawnActorfromClass "/Game/Characters/Singularist/_Core/BP_Singularist.BP_Singularist_C" (CallFunction|FindPlayerStartbyIndex 1) "AlwaysSpawn" "MultiplyWithRoot" 0 0))
      (Pawn|Possess Player%20Controller _returnvalue_3)
      (Development|PrintString "Team 2 player possessed")
      (Development|PrintString (Utilities|GetDisplayName (Pawn|GetControlledPawn Player%20Controller))))))