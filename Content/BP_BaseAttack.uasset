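; Base gameplay ability for an attack with the avatar character's equipped weapon.
; On activation it caches the weapon and plays an attack montage, ending the ability when the montage completes, is interrupted or is cancelled.
; On authority only, it waits for Event.HitScan.Start and End gameplay events, which start and stop the weapon's interval-based hit scan.
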(event Ability|EventActivateAbility
  (bind _asbase_character (Utilities|Casting|CastToBaseCharacter (Ability|GetAvatarActorfromActorInfo))
    (:then
      (Utilities|IsValid _asbase_character
        (:Is%20Valid
          (bind _equippedweapon (Variables|/Script/PROJ.BaseCharacter|GetEquippedWeapon _asbase_character)
            (:then
              (Variables|Default|SetEquipped%20Weapon _equippedweapon)
              (|PlayMontageandWaitProxy "None" (Variables|Default|GetMyMontage) 1.0 "None" true 1.0 0.0 true
                (:then
                  (Ability|HasAuthority
                    (:True
                      (Ability|Tasks|WaitGameplayEvent "(TagName=\"Event.HitScan.Start\")" 0
                        (:then
                          (Ability|Tasks|WaitGameplayEvent "(TagName=\"Event.HitScan.End\")" 0
                            (:EventReceived
                              (bind _equipped_weapon (Variables|Default|GetEquipped%20Weapon)
                                (:then
                                  (Class|Weapon|HitScanEnd _equipped_weapon))
                                (:else)))))
                        (:EventReceived
                          (bind _equipped_weapon_2 (Variables|Default|GetEquipped%20Weapon)
                            (:then
                              (Class|Weapon|HitScanStart _equipped_weapon_2 0.03))
                            (:else)))))))
                (:OnCompleted
                  (Ability|EndAbility :!label _label)
                  (Development|PrintString "Hello"))
                (:OnInterrupted
                  (goto _label))
                (:OnCancelled
                  (goto _label))))
            (:else)))
        (:Is%20Not%20Valid
          (Ability|EndAbility)
          (Development|PrintString "Cast/Valid/Weapon BP_BasicAttack FAILED!"))))
    (:CastFailed
      (Development|PrintString "Hello"))))